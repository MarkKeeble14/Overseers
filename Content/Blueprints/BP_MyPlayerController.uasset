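; Player controller for an auto-battler with a first-person avatar, handling each player's gold, XP, shop, health and mana.
; In planning rounds, input buys, places and sells units through UnitPlacement and SelectLookingAt grid picking; in combat, left click fires a mana-costing autoattack.
; BeginPlay finds the managers, registers a player ID and builds the HUD.
; Tick polls round state to toggle the shop, regenerate resources and refresh the HUD.
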(event Custom|OnTraitAdded
  (params (trait :type ETrait%20Enum :default "T_None"))
  (CallFunction|UpdatePlayerTraitsUI))

(event Custom|OnTraitRemoved
  (params (trait :type ETrait%20Enum :default "T_None"))
  (CallFunction|UpdatePlayerTraitsUI))

(event Input|EnhancedActionEvents|EnhancedInputActionIA_Num1
  (params (ActionValue :type Boolean) (ElapsedSeconds :type Float%20%28double-precision%29) (TriggeredSeconds :type Float%20%28double-precision%29) (InputAction :type Input%20Action%20Object%20Reference :default "/Game/Input/InputActions/NumberKeys/IA_Num1.IA_Num1"))
  (CallFunction|TryPurchaseUnitinShop))

(event Input|EnhancedActionEvents|EnhancedInputActionIA_Test4
  (params (ActionValue :type Boolean) (ElapsedSeconds :type Float%20%28double-precision%29) (TriggeredSeconds :type Float%20%28double-precision%29) (InputAction :type Input%20Action%20Object%20Reference :default "/Game/Input/InputActions/Test/IA_Test4.IA_Test4")))

(event Input|EnhancedActionEvents|EnhancedInputActionIA_Test5
  (params (ActionValue :type Boolean) (ElapsedSeconds :type Float%20%28double-precision%29) (TriggeredSeconds :type Float%20%28double-precision%29) (InputAction :type Input%20Action%20Object%20Reference :default "/Game/Input/InputActions/Test/IA_Test5.IA_Test5")))

(event Input|EnhancedActionEvents|EnhancedInputActionIA_Test6
  (params (ActionValue :type Boolean) (ElapsedSeconds :type Float%20%28double-precision%29) (TriggeredSeconds :type Float%20%28double-precision%29) (InputAction :type Input%20Action%20Object%20Reference :default "/Game/Input/InputActions/Test/IA_Test6.IA_Test6")))

(event Input|EnhancedActionEvents|EnhancedInputActionIA_Test7
  (params (ActionValue :type Boolean) (ElapsedSeconds :type Float%20%28double-precision%29) (TriggeredSeconds :type Float%20%28double-precision%29) (InputAction :type Input%20Action%20Object%20Reference :default "/Game/Input/InputActions/Test/IA_Test7.IA_Test7")))

(event Input|EnhancedActionEvents|EnhancedInputActionIA_Test8
  (params (ActionValue :type Boolean) (ElapsedSeconds :type Float%20%28double-precision%29) (TriggeredSeconds :type Float%20%28double-precision%29) (InputAction :type Input%20Action%20Object%20Reference :default "/Game/Input/InputActions/Test/IA_Test8.IA_Test8")))

(event Input|EnhancedActionEvents|EnhancedInputActionIA_Test9
  (params (ActionValue :type Boolean) (ElapsedSeconds :type Float%20%28double-precision%29) (TriggeredSeconds :type Float%20%28double-precision%29) (InputAction :type Input%20Action%20Object%20Reference :default "/Game/Input/InputActions/Test/IA_Test9.IA_Test9")))

(event Input|EnhancedActionEvents|EnhancedInputActionIA_Num3
  (params (ActionValue :type Boolean) (ElapsedSeconds :type Float%20%28double-precision%29) (TriggeredSeconds :type Float%20%28double-precision%29) (InputAction :type Input%20Action%20Object%20Reference :default "/Game/Input/InputActions/NumberKeys/IA_Num3.IA_Num3"))
  (CallFunction|TryPurchaseUnitinShop 2))

(event Input|EnhancedActionEvents|EnhancedInputActionIA_Num4
  (params (ActionValue :type Boolean) (ElapsedSeconds :type Float%20%28double-precision%29) (TriggeredSeconds :type Float%20%28double-precision%29) (InputAction :type Input%20Action%20Object%20Reference :default "/Game/Input/InputActions/NumberKeys/IA_Num4.IA_Num4"))
  (CallFunction|TryPurchaseUnitinShop 3))

(event Input|EnhancedActionEvents|EnhancedInputActionIA_Num5
  (params (ActionValue :type Boolean) (ElapsedSeconds :type Float%20%28double-precision%29) (TriggeredSeconds :type Float%20%28double-precision%29) (InputAction :type Input%20Action%20Object%20Reference :default "/Game/Input/InputActions/NumberKeys/IA_Num5.IA_Num5"))
  (CallFunction|TryPurchaseUnitinShop 4))

(event Input|EnhancedActionEvents|EnhancedInputActionIA_Num6
  (params (ActionValue :type Boolean) (ElapsedSeconds :type Float%20%28double-precision%29) (TriggeredSeconds :type Float%20%28double-precision%29) (InputAction :type Input%20Action%20Object%20Reference :default "/Game/Input/InputActions/NumberKeys/IA_Num6.IA_Num6")))

(event Input|EnhancedActionEvents|EnhancedInputActionIA_Num7
  (params (ActionValue :type Boolean) (ElapsedSeconds :type Float%20%28double-precision%29) (TriggeredSeconds :type Float%20%28double-precision%29) (InputAction :type Input%20Action%20Object%20Reference :default "/Game/Input/InputActions/NumberKeys/IA_Num7.IA_Num7")))

(event Input|EnhancedActionEvents|EnhancedInputActionIA_Num8
  (params (ActionValue :type Boolean) (ElapsedSeconds :type Float%20%28double-precision%29) (TriggeredSeconds :type Float%20%28double-precision%29) (InputAction :type Input%20Action%20Object%20Reference :default "/Game/Input/InputActions/NumberKeys/IA_Num8.IA_Num8")))

(event Input|EnhancedActionEvents|EnhancedInputActionIA_Num9
  (params (ActionValue :type Boolean) (ElapsedSeconds :type Float%20%28double-precision%29) (TriggeredSeconds :type Float%20%28double-precision%29) (InputAction :type Input%20Action%20Object%20Reference :default "/Game/Input/InputActions/NumberKeys/IA_Num9.IA_Num9")))

(event Input|EnhancedActionEvents|EnhancedInputActionIA_LeftMouseClick
  (params (ActionValue :type Boolean) (ElapsedSeconds :type Float%20%28double-precision%29) (TriggeredSeconds :type Float%20%28double-precision%29) (InputAction :type Input%20Action%20Object%20Reference :default "/Game/Input/InputActions/IA_LeftMouseClick.IA_LeftMouseClick"))
  (bind _unitplacement (Variables|Default|GetUnitPlacement))
  (bind _unitplacement_2 (Variables|Default|GetUnitPlacement))
  (:Triggered
    (Utilities|IsPlanningRound
      (:True
        (Utilities|FlowControl|DoOnce false :!label _label
          (:Completed
            (bind _returnvalue (Class|SelectLookingat|GetSelectedGridCell (Variables|Default|GetSelectLookingAt)))
            (Utilities|IsValid _returnvalue
              (:Is%20Valid
                (bind _returnvalue_2 (Class|UnitPlacement|GetNumUnitsPlaced _unitplacement))
                (bind _returnvalue_3 (Class|UnitPlacement|IsHandEmpty _unitplacement))
                (if _returnvalue_3
                  (Class|UnitPlacement|TryPickupUnit (Variables|Default|GetUnitPlacement) _returnvalue)
                  (else
                    (bind _returnvalue_4 (Class|GridCell|GetCountsTowardUnitMax _returnvalue))
                    (if _returnvalue_4
                      (if (< _returnvalue_2 (Variables|Default|GetMaxUnitsOnBoard))
                        (Class|UnitPlacement|ConfirminHandUnitPlacement _unitplacement_2 _returnvalue))
                      (else
                        (Class|UnitPlacement|ConfirminHandUnitPlacement _unitplacement_2 _returnvalue))))))))))
      (:False
        (bind _asbp_my_character (Utilities|Casting|CastToBP_MyCharacter (Variables|Default|GetMyCharacter)))
        (bind _cost (Default|Autoattack _asbp_my_character))
        (CallFunction|UseMana _cost))))
  (:Completed
    (goto _label Reset)))

(event Input|EnhancedActionEvents|EnhancedInputActionIA_RefreshShop
  (params (ActionValue :type Boolean) (ElapsedSeconds :type Float%20%28double-precision%29) (TriggeredSeconds :type Float%20%28double-precision%29) (InputAction :type Input%20Action%20Object%20Reference :default "/Game/Input/InputActions/IA_RefreshShop.IA_RefreshShop"))
  (bind _refreshshopcost (Variables|Default|GetRefreshShopCost))
  (Utilities|IsPlanningRound
    (:True
      (Utilities|CanPurchase _refreshshopcost
        (:True
          (CallFunction|SubMoney _refreshshopcost)
          (CallFunction|RefreshShop))))))

(event Input|EnhancedActionEvents|EnhancedInputActionIA_LockShop
  (params (ActionValue :type Boolean) (ElapsedSeconds :type Float%20%28double-precision%29) (TriggeredSeconds :type Float%20%28double-precision%29) (InputAction :type Input%20Action%20Object%20Reference :default "/Game/Input/InputActions/IA_LockShop.IA_LockShop"))
  (Utilities|IsPlanningRound
    (:True
      (if (Variables|Default|GetIsShopLocked)
        (Variables|Default|SetIsShopLocked false)
        (else
          (Variables|Default|SetIsShopLocked true))))))

(event Input|EnhancedActionEvents|EnhancedInputActionIA_BuyXP
  (params (ActionValue :type Boolean) (ElapsedSeconds :type Float%20%28double-precision%29) (TriggeredSeconds :type Float%20%28double-precision%29) (InputAction :type Input%20Action%20Object%20Reference :default "/Game/Input/InputActions/IA_BuyXP.IA_BuyXP"))
  (bind _purchasexpcost (Variables|Default|GetPurchaseXPCost))
  (Utilities|CanPurchase _purchasexpcost
    (:True
      (CallFunction|SubMoney _purchasexpcost)
      (CallFunction|AddXP (Variables|Default|GetPurchaseXPAmount)))))

(event Input|EnhancedActionEvents|EnhancedInputActionIA_SellUnit
  (params (ActionValue :type Boolean) (ElapsedSeconds :type Float%20%28double-precision%29) (TriggeredSeconds :type Float%20%28double-precision%29) (InputAction :type Input%20Action%20Object%20Reference :default "/Game/Input/InputActions/IA_SellUnit.IA_SellUnit"))
  (Utilities|IsPlanningRound
    (:True
      (bind _returnvalue (Class|SelectLookingat|GetSelectedGridCell (Variables|Default|GetSelectLookingAt)))
      (Utilities|IsValid _returnvalue
        (:Is%20Valid
          (bind _returnvalue_2 (Class|UnitPlacement|TrySellUnit (Variables|Default|GetUnitPlacement) _returnvalue))
          (if (not (== _returnvalue_2 0))
            (CallFunction|AddMoney _returnvalue_2)))))))

(event Input|EnhancedActionEvents|EnhancedInputActionIA_RightMouseClick
  (params (ActionValue :type Boolean) (ElapsedSeconds :type Float%20%28double-precision%29) (TriggeredSeconds :type Float%20%28double-precision%29) (InputAction :type Input%20Action%20Object%20Reference :default "/Game/Input/InputActions/IA_RightMouseClick.IA_RightMouseClick"))
  (CallFunction|ForceCancelUnitPlacement))

(event Input|EnhancedActionEvents|EnhancedInputActionIA_Num2
  (params (ActionValue :type Boolean) (ElapsedSeconds :type Float%20%28double-precision%29) (TriggeredSeconds :type Float%20%28double-precision%29) (InputAction :type Input%20Action%20Object%20Reference :default "/Game/Input/InputActions/NumberKeys/IA_Num2.IA_Num2"))
  (CallFunction|TryPurchaseUnitinShop 1))

(event Input|EnhancedActionEvents|EnhancedInputActionIA_Test1
  (params (ActionValue :type Boolean) (ElapsedSeconds :type Float%20%28double-precision%29) (TriggeredSeconds :type Float%20%28double-precision%29) (InputAction :type Input%20Action%20Object%20Reference :default "/Game/Input/InputActions/Test/IA_Test1.IA_Test1"))
  (CallFunction|AddMoney 2))

(event Input|EnhancedActionEvents|EnhancedInputActionIA_Test2
  (params (ActionValue :type Boolean) (ElapsedSeconds :type Float%20%28double-precision%29) (TriggeredSeconds :type Float%20%28double-precision%29) (InputAction :type Input%20Action%20Object%20Reference :default "/Game/Input/InputActions/Test/IA_Test2.IA_Test2"))
  (Class|RoundManager|BeginGame (Variables|Default|GetRoundManager)))

(event Input|EnhancedActionEvents|EnhancedInputActionIA_Test3
  (params (ActionValue :type Boolean) (ElapsedSeconds :type Float%20%28double-precision%29) (TriggeredSeconds :type Float%20%28double-precision%29) (InputAction :type Input%20Action%20Object%20Reference :default "/Game/Input/InputActions/Test/IA_Test3.IA_Test3")))

(event EventBeginPlay
  (Utilities|FlowControl|DelayUntilNextTick)
  (CallFunction|SetupInputMappingContext)
  (CallFunction|InitializePlayer)
  (EventDispatchers|BindEventtoOnTraitAddedtoBoard (delegate Custom|OnTraitAdded))
  (EventDispatchers|BindEventtoOnTraitRemovedfromBoard (delegate Custom|OnTraitRemoved))
  (CallFunction|SetupUI))

(event Collision|EventActorBeginOverlap
  (params (OtherActor :type Actor%20Object%20Reference)))

(event EventTick
  (params (DeltaSeconds :type Float%20%28single-precision%29))
  (Utilities|IsValid (Variables|Default|GetPlayerHUD)
    (:Is%20Valid
      (CallFunction|RegenerateMana DeltaSeconds)
      (Class|ResourceContainer|AlterResource (Variables|Default|GetHealth) (Variables|Default|GetHealthRegen))
      (CallFunction|SetAllowSelect)
      (CallFunction|SetShopState)
      (CallFunction|SetCrosshairState)
      (CallFunction|UpdateRoundText)
      (CallFunction|SetUnitsonBoardText)
      (CallFunction|SetHUDBars))))

(fn ConstructionScript)

(fn GetUnitinShopatIndex
  (params (Index :type Integer))
  (return (Utilities|ResolveSoftReference (Utilities|Array|Get(acopy) (Variables|Default|GetUnitsInShop) Index))))

(fn SetUnitsinShop
  (bind _availableunits (Variables|Default|GetAvailableUnits))
  (for _index (range 0 4)
    (Utilities|Array|Add (Variables|Default|GetUnitsInShop) (Utilities|Array|Get(acopy) _availableunits (Math|Random|RandomIntegerinRange 0 (- (Utilities|Array|Length _availableunits) 1)))))
  (for (_array_element _array_index) (Variables|Default|GetUnitsInShop)
    (Default|SetShopItem (Variables|Default|GetPlayerHUD) _array_element (+ _array_index 1))))

(fn ClearShop
  (Default|ClearShopSlots (Variables|Default|GetPlayerHUD))
  (Utilities|Array|Clear (Variables|Default|GetUnitsInShop)))

(fn RefreshShop
  (if (not (Variables|Default|GetIsShopLocked))
    (CallFunction|ClearShop)
    (CallFunction|SetUnitsinShop)))

(fn OpenShop
  (params (HUD :type WBP%20Player%20HUD%20Object%20Reference))
  (Default|SetShopVisibility HUD "Visible")
  (Variables|Default|SetIsShopOpen true))

(fn CloseShop
  (params (HUD :type WBP%20Player%20HUD%20Object%20Reference))
  (Default|SetShopVisibility HUD "Collapsed")
  (Variables|Default|SetIsShopOpen false))

(fn SetMoneyText
  (Default|SetCurrentMoneyText (Variables|Default|GetPlayerHUD) (Utilities|Text|ToText(Integer) (.m_CurrentGold (Utilities|Struct|BreakPlayerInfo (Variables|Default|GetPlayerInfo))))))

(fn SetXPText
  (bind _playerinfo (Variables|Default|GetPlayerInfo))
  (bind (_m_playerlevel _m_currentxp _m_xpforlevelup) (Utilities|Struct|BreakPlayerInfo _playerinfo))
  (Default|SetCurrentLevelText (Variables|Default|GetPlayerHUD) (Utilities|Text|FormatText "{CurrentXP} / {NextLevelXP} : {Level}" _m_currentxp _m_xpforlevelup _m_playerlevel)))

(fn SetUnitsonBoardText
  (bind _returnvalue (Class|UnitPlacement|GetNumUnitsPlaced (Variables|Default|GetUnitPlacement)))
  (Default|SetUnitsonBoardText (Variables|Default|GetPlayerHUD) (Utilities|Text|FormatText "{CurrentUnits} / {MaxUnits}" _returnvalue (Variables|Default|GetMaxUnitsOnBoard))))

(fn LevelUp
  (bind _playerinfo (Variables|Default|GetPlayerInfo))
  (bind (_m_playerlevel _m_currentxp _m_xpforlevelup) (Utilities|Struct|BreakPlayerInfo _playerinfo))
  (bind _structout (Utilities|Struct|SetmembersinPlayerInfo _playerinfo (+ _m_playerlevel 1) (- _m_currentxp _m_xpforlevelup)))
  (Math|Integer|IncrementInt (Variables|Default|GetMaxUnitsOnBoard)
    (:%20%20
      (CallFunction|SetUnitsonBoardText)
      (Utilities|Struct|SetmembersinPlayerInfo _structout (+ _m_xpforlevelup 5))
      (return))))

(fn AddXP
  (params (XPGained :type Integer))
  (bind _playerinfo (Variables|Default|GetPlayerInfo))
  (Utilities|Struct|SetmembersinPlayerInfo _playerinfo (+ XPGained (.m_CurrentXP (Utilities|Struct|BreakPlayerInfo _playerinfo))))
  (Utilities|ShouldLevelUp
    (:True
      (CallFunction|LevelUp))
    (:False
      _))
  (CallFunction|SetXPText))

(fn AddMoney
  (params (Amount :type Integer))
  (bind _playerinfo (Variables|Default|GetPlayerInfo))
  (Utilities|Struct|SetmembersinPlayerInfo _playerinfo (+ (.m_CurrentGold (Utilities|Struct|BreakPlayerInfo _playerinfo)) Amount))
  (CallFunction|SetMoneyText))

(fn SubMoney
  (params (Amount :type Integer))
  (bind _playerinfo (Variables|Default|GetPlayerInfo))
  (Utilities|Struct|SetmembersinPlayerInfo _playerinfo (- (.m_CurrentGold (Utilities|Struct|BreakPlayerInfo _playerinfo)) Amount))
  (CallFunction|SetMoneyText))

(fn TryPurchaseUnitinShop
  (params (Index :type Integer))
  (Utilities|IsPlanningRound
    (:True
      (bind _asmy_character (CallFunction|GetMyCharacterReference))
      (bind _returnvalue (Class|MyCharacter|GetPlayerMode _asmy_character))
      (switch int _returnvalue
        (:1
          _)
        (:2
          _)
        (:3
          _))
      (bind _class (CallFunction|GetUnitinShopatIndex Index))
      (bind _returnvalue_2 (Game|SpawnActorfromClass _class (Math|Transform|MakeTransform "0, 0, 0" "0, 0, 0" "0.000000,0.000000,0.000000") "Undefined" "MultiplyWithRoot" 0 0))
      (bind _returnvalue_3 (Class|Unit|GetData _returnvalue_2))
      (Actor|DestroyActor _returnvalue_2)
      (Utilities|CanPurchase (.m_Rarity (Utilities|Struct|BreakUnitInfo _returnvalue_3))
        (:True
          (CallFunction|SubMoney (.m_Rarity (Utilities|Struct|BreakUnitInfo _returnvalue_3)))
          (bind _returnvalue_4 (Class|UnitPlacement|CreateUnit (Variables|Default|GetUnitPlacement) _class))
          (bind _asunit (Utilities|Casting|CastToUnit _returnvalue_4))
          (return _asunit))))))

(fn ForceCancelUnitPlacement
  (bind _returnvalue (Class|UnitPlacement|CancelinHandUnitPlacement (Variables|Default|GetUnitPlacement)))
  (CallFunction|AddMoney _returnvalue))

(fn UpdatePlayerTraitsUI
  (bind _returnvalue (Class|MyPlayerController|GetPlayerId))
  (bind _returnvalue_2 (Class|GridManager|GetCopyOfPlayerBoardData (Variables|Default|GetGridManager) _returnvalue))
  (Default|SetPlayerTraitsUI (Variables|Default|GetPlayerHUD) (Utilities|Struct|BreakBoardData _returnvalue_2) (Variables|Default|GetTraitsManager)))

(fn SetupInputMappingContext
  (bind _self self)
  (bind _returnvalue (PlayerController|LocalPlayerSubsystems|GetEnhancedInputLocalPlayerSubsystem _self))
  (Utilities|IsValid _returnvalue
    (:Is%20Valid
      (Input|AddMappingContext _returnvalue "/Game/Input/IMC_Gameplay.IMC_Gameplay" 0 "(bIgnoreAllPressedKeysUntilRelease=True,bForceImmediately=False,bNotifyUserSettings=False)"))))

(fn InitializePlayer
  (bind _self self)
  (Utilities|FlowControl|Sequence
    (:then_0
      (bind _asmy_character (CallFunction|GetMyCharacterReference))
      (Variables|Default|SetMyCharacter _asmy_character))
    (:then_1
      (bind _returnvalue (Actor|GetActorOfClass "/Game/Blueprints/Gameplay/Managers/BP_RoundManager.BP_RoundManager_C"))
      (Variables|Default|SetRoundManager _returnvalue))
    (:then_2
      (bind _returnvalue_2 (Actor|GetActorOfClass "/Game/Blueprints/Gameplay/Managers/BP_MyNetworkManager.BP_MyNetworkManager_C"))
      (bind _output_get (Variables|Default|SetNetworkManager _returnvalue_2)))
    (:then_3
      (bind _returnvalue_3 (Actor|GetActorOfClass "/Game/Blueprints/Gameplay/Managers/BP_GridManager.BP_GridManager_C"))
      (bind _output_get_2 (Variables|Default|SetGridManager _returnvalue_3))
      (Class|MyPlayerController|SetGridManager _output_get_2)
      (Class|GridManager|SetCharacterBounds _output_get_2 (Variables|Default|GetMyCharacter)))
    (:then_4
      (bind _returnvalue_4 (Actor|GetActorOfClass "/Game/Blueprints/Gameplay/Managers/BP_TraitsManager.BP_TraitsManager_C"))
      (bind _output_get_3 (Variables|Default|SetTraitsManager _returnvalue_4))
      (Class|MyPlayerController|SetTraitsManager _output_get_3))
    (:then_5
      (bind _returnvalue_5 (Class|MyNetworkManager|GetNextPlayerIndex _output_get))
      (Class|MyPlayerController|SetPlayerId _returnvalue_5)
      (Class|MyNetworkManager|IncrementNextPlayerIndex _output_get)
      (Class|GridManager|AttachPlayertoBoardData (Variables|Default|GetGridManager) _returnvalue_5 self)
      (bind _asmy_character_2 (CallFunction|GetMyCharacterReference))
      (bind _asbp_my_character (Utilities|Casting|CastToBP_MyCharacter _asmy_character_2))
      (Default|SetPlayerInitPosition _asbp_my_character _returnvalue_5)
      (Class|SelectLookingat|SetSelectingfor (Variables|Default|GetSelectLookingAt) _self)
      (Class|UnitPlacement|SetPlacingfor (Variables|Default|GetUnitPlacement) _self)
      (return _returnvalue_5))))

(fn SetupUI
  (if (Pawn|IsLocalPlayerController)
    (bind _returnvalue (UserInterface|CreateWidget "/Game/Blueprints/UI/WBP_PlayerHUD.WBP_PlayerHUD_C"))
    (bind _output_get (Variables|Default|SetPlayerHUD _returnvalue))
    (UserInterface|Viewport|AddtoViewport _output_get 0)
    (CallFunction|SetUnitsinShop)
    (CallFunction|OpenShop _output_get)
    (CallFunction|SetMoneyText)
    (Utilities|Struct|SetmembersinPlayerInfo (Variables|Default|GetPlayerInfo) (Variables|Default|GetXPForLevel))
    (CallFunction|SetXPText)
    (CallFunction|SetUnitsonBoardText)))

(fn SetAllowSelect
  (bind _selectlookingat (Variables|Default|GetSelectLookingAt))
  (bind _returnvalue (Class|MyCharacter|GetPlayerMode (Variables|Default|GetMyCharacter)))
  (switch int _returnvalue
    (:0
      (Class|SelectLookingat|SetAllowSelect _selectlookingat false :!label _label))
    (:1
      (Class|SelectLookingat|SetAllowSelect _selectlookingat true))
    (:2
      (goto _label))
    (:3
      (goto _label))))

(fn SetCrosshairState
  (bind _returnvalue (Actor|GetComponentbyClass "/Script/Overseers.SelectLookingAt"))
  (bind _playerhud (Variables|Default|GetPlayerHUD))
  (Utilities|IsValid _returnvalue
    (:Is%20Valid
      (bind _returnvalue_2 (Class|SelectLookingat|HasSomethingSelected _returnvalue))
      (if _returnvalue_2
        (Default|SetCenterColor _playerhud (Variables|Default|GetCrosshairCenterColorSelected))
        (else
          (Default|SetCenterColor _playerhud (Variables|Default|GetCrosshairCenterColorNotSelected)))))))

(fn UpdateRoundText
  (bind _playerhud (Variables|Default|GetPlayerHUD))
  (bind _roundmanager (Variables|Default|GetRoundManager))
  (bind _returnvalue (Class|RoundManager|GetCurrentRoundType _roundmanager))
  (Default|SetRoundTypeText _playerhud (Utilities|Text|ToText(String) (Utilities|String|EnumtoString _returnvalue)))
  (bind _returnvalue_2 (Class|RoundManager|GetPlanningRoundTimer _roundmanager))
  (if (<= _returnvalue_2 0.0)
    (Default|SetPlanningPhaseTimerText _playerhud)
    (else
      (Default|SetPlanningPhaseTimerText _playerhud (Utilities|Text|ToText(Integer) (Math|Float|Round _returnvalue_2))))))

(fn SetShopState
  (bind _playerhud (Variables|Default|GetPlayerHUD))
  (Utilities|IsPlanningRound
    (:True
      (CallFunction|OpenShop _playerhud))
    (:False
      (CallFunction|CloseShop _playerhud)
      (CallFunction|ForceCancelUnitPlacement))))

(fn SetHUDBars
  (bind _playerhud (Variables|Default|GetPlayerHUD))
  (bind _returnvalue (Class|ResourceContainer|GetPercent (Variables|Default|GetHealth)))
  (Default|SetHPBarPercent _playerhud _returnvalue)
  (bind _returnvalue_2 (Class|ResourceContainer|GetPercent (Variables|Default|GetMana)))
  (Default|SetManaBarPercent _playerhud _returnvalue_2))

(fn RegenerateMana
  (params (DeltaTime :type Float%20%28double-precision%29))
  (if (<= (Variables|Default|GetManaRegenDelayTimer) 0.0)
    (Class|ResourceContainer|AlterResource (Variables|Default|GetMana) (Variables|Default|GetManaRegen))
    (else
      (Variables|Default|SetManaRegenDelayTimer (- (Variables|Default|GetManaRegenDelayTimer) DeltaTime)))))

(fn UseMana
  (params (A :type Float%20%28double-precision%29))
  (Class|ResourceContainer|AlterResource (Variables|Default|GetMana) (* A -1.0))
  (Variables|Default|SetManaRegenDelayTimer (Variables|Default|GetManaRegenDelay)))

(fn GetMyCharacterReference
  (bind _asmy_character (Utilities|Casting|CastToMyCharacter (Pawn|GetControlledPawn))
    (:then
      _)
    (:CastFailed
      _))
  (return _asmy_character))