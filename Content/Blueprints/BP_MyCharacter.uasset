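; Player character that moves, buys units from a random shop and places them in the world.
; BeginPlay adds Enhanced Input, creates the HUD and rolls five shop units from AvailableUnits; test inputs show, hide or reroll the shop.
; Number keys create shop units through UnitPlacement, and clicks pick up or confirm placement.
; Tick interpolates camera FOV by player mode and sprint, and tints the crosshair when SelectLookingAt has a selection.
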(event Input|EnhancedActionEvents|EnhancedInputActionIA_Jump
  (params (ActionValue :type Boolean) (ElapsedSeconds :type Float%20%28double-precision%29) (TriggeredSeconds :type Float%20%28double-precision%29) (InputAction :type Input%20Action%20Object%20Reference :default "/Game/Input/InputActions/IA_Jump.IA_Jump"))
  (Class|MyCharacter|CallJump))

(event Input|EnhancedActionEvents|EnhancedInputActionIA_Num1
  (params (ActionValue :type Boolean) (ElapsedSeconds :type Float%20%28double-precision%29) (TriggeredSeconds :type Float%20%28double-precision%29) (InputAction :type Input%20Action%20Object%20Reference :default "/Game/Input/InputActions/NumberKeys/IA_Num1.IA_Num1"))
  (bind _class (CallFunction|GetUnitinShopatIndex))
  (Class|UnitPlacement|CreateUnit (Variables|Default|GetUnitPlacement) _class))

(event Input|EnhancedActionEvents|EnhancedInputActionIA_Test4
  (params (ActionValue :type Boolean) (ElapsedSeconds :type Float%20%28double-precision%29) (TriggeredSeconds :type Float%20%28double-precision%29) (InputAction :type Input%20Action%20Object%20Reference :default "/Game/Input/InputActions/Test/IA_Test4.IA_Test4")))

(event Input|EnhancedActionEvents|EnhancedInputActionIA_Test5
  (params (ActionValue :type Boolean) (ElapsedSeconds :type Float%20%28double-precision%29) (TriggeredSeconds :type Float%20%28double-precision%29) (InputAction :type Input%20Action%20Object%20Reference :default "/Game/Input/InputActions/Test/IA_Test5.IA_Test5")))

(event Input|EnhancedActionEvents|EnhancedInputActionIA_Test6
  (params (ActionValue :type Boolean) (ElapsedSeconds :type Float%20%28double-precision%29) (TriggeredSeconds :type Float%20%28double-precision%29) (InputAction :type Input%20Action%20Object%20Reference :default "/Game/Input/InputActions/Test/IA_Test6.IA_Test6")))

(event Input|EnhancedActionEvents|EnhancedInputActionIA_Test7
  (params (ActionValue :type Boolean) (ElapsedSeconds :type Float%20%28double-precision%29) (TriggeredSeconds :type Float%20%28double-precision%29) (InputAction :type Input%20Action%20Object%20Reference :default "/Game/Input/InputActions/Test/IA_Test7.IA_Test7")))

(event Input|EnhancedActionEvents|EnhancedInputActionIA_Test8
  (params (ActionValue :type Boolean) (ElapsedSeconds :type Float%20%28double-precision%29) (TriggeredSeconds :type Float%20%28double-precision%29) (InputAction :type Input%20Action%20Object%20Reference :default "/Game/Input/InputActions/Test/IA_Test8.IA_Test8")))

(event Input|EnhancedActionEvents|EnhancedInputActionIA_Test9
  (params (ActionValue :type Boolean) (ElapsedSeconds :type Float%20%28double-precision%29) (TriggeredSeconds :type Float%20%28double-precision%29) (InputAction :type Input%20Action%20Object%20Reference :default "/Game/Input/InputActions/Test/IA_Test9.IA_Test9")))

(event Input|EnhancedActionEvents|EnhancedInputActionIA_BeginSprint
  (params (ActionValue :type Boolean) (ElapsedSeconds :type Float%20%28double-precision%29) (TriggeredSeconds :type Float%20%28double-precision%29) (InputAction :type Input%20Action%20Object%20Reference :default "/Game/Input/InputActions/IA_BeginSprint.IA_BeginSprint"))
  (Class|MyCharacter|StartSprint))

(event Input|EnhancedActionEvents|EnhancedInputActionIA_Num3
  (params (ActionValue :type Boolean) (ElapsedSeconds :type Float%20%28double-precision%29) (TriggeredSeconds :type Float%20%28double-precision%29) (InputAction :type Input%20Action%20Object%20Reference :default "/Game/Input/InputActions/NumberKeys/IA_Num3.IA_Num3"))
  (bind _class (CallFunction|GetUnitinShopatIndex 2))
  (Class|UnitPlacement|CreateUnit (Variables|Default|GetUnitPlacement) _class))

(event Input|EnhancedActionEvents|EnhancedInputActionIA_Look
  (params (ActionValue :type Vector%202D%20Structure) (ElapsedSeconds :type Float%20%28double-precision%29) (TriggeredSeconds :type Float%20%28double-precision%29) (InputAction :type Input%20Action%20Object%20Reference :default "/Game/Input/InputActions/IA_Look.IA_Look"))
  (bind (_x _y) (Math|Vector2D|BreakVector2D ActionValue))
  (Pawn|Input|AddControllerPitchInput (* _y -1.0))
  (Pawn|Input|AddControllerYawInput _x))

(event Input|EnhancedActionEvents|EnhancedInputActionIA_EndSprint
  (params (ActionValue :type Boolean) (ElapsedSeconds :type Float%20%28double-precision%29) (TriggeredSeconds :type Float%20%28double-precision%29) (InputAction :type Input%20Action%20Object%20Reference :default "/Game/Input/InputActions/IA_EndSprint.IA_EndSprint"))
  (Class|MyCharacter|StopSprint))

(event Input|EnhancedActionEvents|EnhancedInputActionIA_BeginCrouch
  (params (ActionValue :type Boolean) (ElapsedSeconds :type Float%20%28double-precision%29) (TriggeredSeconds :type Float%20%28double-precision%29) (InputAction :type Input%20Action%20Object%20Reference :default "/Game/Input/InputActions/IA_BeginCrouch.IA_BeginCrouch"))
  (Character|Crouch)
  (Class|MyCharacter|StartCrouch))

(event Input|EnhancedActionEvents|EnhancedInputActionIA_Num4
  (params (ActionValue :type Boolean) (ElapsedSeconds :type Float%20%28double-precision%29) (TriggeredSeconds :type Float%20%28double-precision%29) (InputAction :type Input%20Action%20Object%20Reference :default "/Game/Input/InputActions/NumberKeys/IA_Num4.IA_Num4"))
  (bind _class (CallFunction|GetUnitinShopatIndex 3))
  (Class|UnitPlacement|CreateUnit (Variables|Default|GetUnitPlacement) _class))

(event Input|EnhancedActionEvents|EnhancedInputActionIA_Num5
  (params (ActionValue :type Boolean) (ElapsedSeconds :type Float%20%28double-precision%29) (TriggeredSeconds :type Float%20%28double-precision%29) (InputAction :type Input%20Action%20Object%20Reference :default "/Game/Input/InputActions/NumberKeys/IA_Num5.IA_Num5"))
  (bind _class (CallFunction|GetUnitinShopatIndex 4))
  (Class|UnitPlacement|CreateUnit (Variables|Default|GetUnitPlacement) _class))

(event Input|EnhancedActionEvents|EnhancedInputActionIA_Num6
  (params (ActionValue :type Boolean) (ElapsedSeconds :type Float%20%28double-precision%29) (TriggeredSeconds :type Float%20%28double-precision%29) (InputAction :type Input%20Action%20Object%20Reference :default "/Game/Input/InputActions/NumberKeys/IA_Num6.IA_Num6")))

(event Input|EnhancedActionEvents|EnhancedInputActionIA_Num7
  (params (ActionValue :type Boolean) (ElapsedSeconds :type Float%20%28double-precision%29) (TriggeredSeconds :type Float%20%28double-precision%29) (InputAction :type Input%20Action%20Object%20Reference :default "/Game/Input/InputActions/NumberKeys/IA_Num7.IA_Num7")))

(event Input|EnhancedActionEvents|EnhancedInputActionIA_Num8
  (params (ActionValue :type Boolean) (ElapsedSeconds :type Float%20%28double-precision%29) (TriggeredSeconds :type Float%20%28double-precision%29) (InputAction :type Input%20Action%20Object%20Reference :default "/Game/Input/InputActions/NumberKeys/IA_Num8.IA_Num8")))

(event Input|EnhancedActionEvents|EnhancedInputActionIA_Num9
  (params (ActionValue :type Boolean) (ElapsedSeconds :type Float%20%28double-precision%29) (TriggeredSeconds :type Float%20%28double-precision%29) (InputAction :type Input%20Action%20Object%20Reference :default "/Game/Input/InputActions/NumberKeys/IA_Num9.IA_Num9")))

(event Input|EnhancedActionEvents|EnhancedInputActionIA_MouseClick
  (params (ActionValue :type Boolean) (ElapsedSeconds :type Float%20%28double-precision%29) (TriggeredSeconds :type Float%20%28double-precision%29) (InputAction :type Input%20Action%20Object%20Reference :default "/Game/Input/InputActions/IA_MouseClick.IA_MouseClick"))
  (bind _unitplacement (Variables|Default|GetUnitPlacement))
  (bind _returnvalue (Class|UnitPlacement|IsHandEmpty _unitplacement))
  (if _returnvalue
    (Class|UnitPlacement|PickupUnit _unitplacement)
    (else
      (Class|UnitPlacement|ConfirminHandUnitPlacement _unitplacement))))

(event Input|EnhancedActionEvents|EnhancedInputActionIA_ToggleMode
  (params (ActionValue :type Boolean) (ElapsedSeconds :type Float%20%28double-precision%29) (TriggeredSeconds :type Float%20%28double-precision%29) (InputAction :type Input%20Action%20Object%20Reference :default "/Game/Input/InputActions/IA_ToggleMode.IA_ToggleMode"))
  (Class|MyCharacter|ToggleMode))

(event Input|EnhancedActionEvents|EnhancedInputActionIA_Num2
  (params (ActionValue :type Boolean) (ElapsedSeconds :type Float%20%28double-precision%29) (TriggeredSeconds :type Float%20%28double-precision%29) (InputAction :type Input%20Action%20Object%20Reference :default "/Game/Input/InputActions/NumberKeys/IA_Num2.IA_Num2"))
  (bind _class (CallFunction|GetUnitinShopatIndex 1))
  (Class|UnitPlacement|CreateUnit (Variables|Default|GetUnitPlacement) _class))

(event Input|EnhancedActionEvents|EnhancedInputActionIA_Move
  (params (ActionValue :type Vector%202D%20Structure) (ElapsedSeconds :type Float%20%28double-precision%29) (TriggeredSeconds :type Float%20%28double-precision%29) (InputAction :type Input%20Action%20Object%20Reference :default "/Game/Input/InputActions/IA_Move.IA_Move"))
  (bind (_x _y) (Math|Vector2D|BreakVector2D ActionValue))
  (Class|MyCharacter|MoveRight _x)
  (Class|MyCharacter|MoveForward _y))

(event Input|EnhancedActionEvents|EnhancedInputActionIA_EndCrouch
  (params (ActionValue :type Boolean) (ElapsedSeconds :type Float%20%28double-precision%29) (TriggeredSeconds :type Float%20%28double-precision%29) (InputAction :type Input%20Action%20Object%20Reference :default "/Game/Input/InputActions/IA_EndCrouch.IA_EndCrouch"))
  (Character|UnCrouch)
  (Class|MyCharacter|StopCrouch))

(event Input|EnhancedActionEvents|EnhancedInputActionIA_Test1
  (params (ActionValue :type Boolean) (ElapsedSeconds :type Float%20%28double-precision%29) (TriggeredSeconds :type Float%20%28double-precision%29) (InputAction :type Input%20Action%20Object%20Reference :default "/Game/Input/InputActions/Test/IA_Test1.IA_Test1"))
  (Default|SetShopVisibility (Variables|Default|GetPlayerHUD) "Visible")
  (Variables|Default|SetIsShopOpen true))

(event Input|EnhancedActionEvents|EnhancedInputActionIA_Test2
  (params (ActionValue :type Boolean) (ElapsedSeconds :type Float%20%28double-precision%29) (TriggeredSeconds :type Float%20%28double-precision%29) (InputAction :type Input%20Action%20Object%20Reference :default "/Game/Input/InputActions/Test/IA_Test2.IA_Test2"))
  (Default|SetShopVisibility (Variables|Default|GetPlayerHUD) "Collapsed")
  (Variables|Default|SetIsShopOpen false))

(event Input|EnhancedActionEvents|EnhancedInputActionIA_Test3
  (params (ActionValue :type Boolean) (ElapsedSeconds :type Float%20%28double-precision%29) (TriggeredSeconds :type Float%20%28double-precision%29) (InputAction :type Input%20Action%20Object%20Reference :default "/Game/Input/InputActions/Test/IA_Test3.IA_Test3"))
  (CallFunction|RefreshShop))

(event EventBeginPlay
  (bind _asplayer_controller (Utilities|Casting|CastToPlayerController (Pawn|GetController)))
  (Utilities|IsValid (PlayerController|LocalPlayerSubsystems|GetEnhancedInputLocalPlayerSubsystem _asplayer_controller)
    (:Is%20Valid
      (Variables|Default|SetPlayerController _asplayer_controller)
      (Input|AddMappingContext (PlayerController|LocalPlayerSubsystems|GetEnhancedInputLocalPlayerSubsystem _asplayer_controller) "/Game/Input/IMC_Gameplay.IMC_Gameplay" 0 "(bIgnoreAllPressedKeysUntilRelease=True,bForceImmediately=False,bNotifyUserSettings=False)")
      (bind _returnvalue (UserInterface|CreateWidget "/Game/Blueprints/UI/WBP_PlayerHUD.WBP_PlayerHUD_C"))
      (bind _output_get (Variables|Default|SetPlayerHUD _returnvalue))
      (UserInterface|Viewport|AddtoViewport _output_get 0)
      (CallFunction|SetUnitsinShop))))

(event Collision|EventActorBeginOverlap
  (params (OtherActor :type Actor%20Object%20Reference)))

(event EventTick
  (params (DeltaSeconds :type Float%20%28single-precision%29))
  (bind _returnvalue (Actor|GetComponentbyClass "/Script/Overseers.SelectLookingAt"))
  (bind _returnvalue_2 (Class|MyCharacter|GetPlayerMode))
  (switch int _returnvalue_2
    (:0
      (bind _returnvalue_3 (Class|MyCharacter|GetIsSprinting :!label _label))
      (CallFunction|SetFOV (select _returnvalue_3 (Variables|Default|GetSprintingFOV) (Variables|Default|GetDefaultFOV)))
      (Utilities|IsValid _returnvalue
        (:Is%20Valid
          (bind _returnvalue_4 (Class|SelectLookingat|HasSomethingSelected _returnvalue)))))
    (:1
      (goto _label))
    (:2
      (CallFunction|SetFOV (Variables|Default|GetPlayerModeTransitionFOV) :!label _label_2))
    (:3
      (goto _label_2)))
  (if _returnvalue_4
    (Default|SetCenterColor (stale EventBeginPlay _returnvalue) (Variables|Default|GetCrosshairCenterColorSelected))
    (else
      (Default|SetCenterColor (stale EventBeginPlay _returnvalue) (Variables|Default|GetCrosshairCenterColorNotSelected)))))

(fn ConstructionScript)

(fn SetFOV
  (params (Target :type Float%20%28double-precision%29))
  (Camera|SetFieldOfView (Variables|Default|GetCamera) (Math|Interpolation|FInterpTo (Variables|/Script/Engine.CameraComponent|GetFieldOfView (Variables|Default|GetCamera)) Target (Utilities|Time|GetWorldDeltaSeconds) (Variables|Default|GetFOVInterpolationSpeed))))

(fn GetUnitinShopatIndex
  (params (Index :type Integer))
  (return (.Class (Utilities|Struct|BreakUnitData (Utilities|Array|Get(acopy) (Variables|Default|GetUnitsInShop) Index)))))

(fn SetUnitsinShop
  (bind _availableunits (Variables|Default|GetAvailableUnits))
  (for _index (range 0 4)
    (Utilities|Array|Add (Variables|Default|GetUnitsInShop) (Utilities|Array|Get(acopy) _availableunits (Math|Random|RandomIntegerinRange 0 (- (Utilities|Array|Length _availableunits) 1)))))
  (for (_array_element _array_index) (Variables|Default|GetUnitsInShop)
    (Default|SetShopItem (Variables|Default|GetPlayerHUD) _array_element (+ _array_index 1))))

(fn ClearShop
  (Default|ClearShopSlots (Variables|Default|GetPlayerHUD))
  (Utilities|Array|Clear (Variables|Default|GetUnitsInShop)))

(fn RefreshShop
  (CallFunction|ClearShop)
  (CallFunction|SetUnitsinShop))