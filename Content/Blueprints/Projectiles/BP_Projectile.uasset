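; BP_Projectile is a projectile actor that destroys itself on any hit or 15 seconds after spawning.
; BeginPlay applies a uniform start scale, then Tick sets scale to a lerp between start and max using LerpSpeed as a constant alpha, giving a fixed size rather than progressive growth.
; Hit checks for a "Damagable" tag, but both branches are empty, so no damage is applied.
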(event EventBeginPlay
  (bind _startscale (Variables|Default|GetStartScale))
  (Transformation|SetActorScale3D (Math|Vector|MakeVector _startscale _startscale _startscale))
  (Utilities|FlowControl|Delay 15.0)
  (Actor|DestroyActor))

(event Collision|EventActorBeginOverlap
  (params (OtherActor :type Actor%20Object%20Reference)))

(event EventTick
  (params (DeltaSeconds :type Float%20%28single-precision%29))
  (bind _maxscale (Variables|Default|GetMaxScale))
  (bind _startscale (Variables|Default|GetStartScale))
  (Transformation|SetActorScale3D (Math|Vector|Lerp(Vector) (Math|Vector|MakeVector _startscale _startscale _startscale) (Math|Vector|MakeVector _maxscale _maxscale _maxscale) (Variables|Default|GetLerpSpeed))))

(event Collision|EventHit
  (params (MyComp :type Primitive%20Component%20Object%20Reference) (Other :type Actor%20Object%20Reference) (OtherComp :type Primitive%20Component%20Object%20Reference) (bSelfMoved :type Boolean) (HitLocation :type Vector :default "0, 0, 0") (HitNormal :type Vector :default "0, 0, 0") (NormalImpulse :type Vector :default "0, 0, 0") (Hit :type Hit%20Result%20Structure%20%28by%20ref%29))
  (if (Actor|ActorHasTag Other "Damagable")
    _
    (else
      _))
  (Actor|DestroyActor))

(fn ConstructionScript)