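; Base player character that switches between grounded movement with sprint, crouch and jump, and an aerial Oversight mode.
; Toggling passes through Rising, an authority-driven ascent to a set height, or Falling, a downward launch until landing, with Tick adjusting gravity per mode.
; Oversight movement sets location directly within X/Y bounds, while sprint's RepNotify updates walk speed.
; FOV, camera shake and mesh visibility helpers use hardcoded conditions and are not called here.
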(event Custom|SetupInputMappingContext
  (params (PlayerController :type Player%20Controller%20Object%20Reference))
  (bind _returnvalue (PlayerController|LocalPlayerSubsystems|GetEnhancedInputLocalPlayerSubsystem PlayerController))
  ;[1 1 1] Setup Input
  (Utilities|IsValid _returnvalue
    (:Is%20Valid
      (Input|AddMappingContext _returnvalue "/Game/Input/IMC_Character.IMC_Character" 0 "(bIgnoreAllPressedKeysUntilRelease=True,bForceImmediately=False,bNotifyUserSettings=False)"))))

(event Custom|StartCrouch
  ;[1 1 1] Handles crouching
  (if (Utilities|Enum|Equal(Enum) (Variables|ModeInfo|GetPlayerMode) "NewEnumerator2")
    (Character|Crouch)))

(event Custom|ToggleMode
  (bind _charactermovement (Variables|Character|GetCharacterMovement))
  (switch Utilities|FlowControl|Switch|SwitchonCharacterMode (Variables|ModeInfo|GetPlayerMode)
    (:NewEnumerator0
      (Variables|Movement|SetIsSprinting false)
      (Variables|/Script/Engine.MovementComponent|SetVelocity _charactermovement "0, 0, 0")
      (Variables|ModeInfo|SetPlayerMode "NewEnumerator1")
      (Character|LaunchCharacter (Math|Vector|MakeVector 0.0 0.0 (Variables|Oversight|GetDescendLaunchingForce)) true true))
    (:NewEnumerator2
      (Variables|Movement|SetIsSprinting false)
      (Variables|/Script/Engine.MovementComponent|SetVelocity _charactermovement "0, 0, 0")
      (Variables|ModeInfo|SetPlayerMode "NewEnumerator3"))))

(event Custom|UpdateActorLocation
  (params (NewLocation :type Vector))
  (Transformation|SetActorLocation NewLocation false false))

(event Custom|RiseToOversight
  (params (DeltaTime :type Float%20%28double-precision%29))
  (bind _returnvalue (Transformation|GetActorLocation))
  (bind _ascendspeed (Variables|Oversight|GetAscendSpeed))
  (bind _returnvalue_2 (* _ascendspeed DeltaTime))
  (bind _returnvalue_3 (+ _returnvalue (Math|Vector|MakeVector 0.0 0.0 _returnvalue_2)))
  (Transformation|SetActorLocation _returnvalue_3 false false)
  (CallFunction|UpdateActorLocation _returnvalue_3))

(event Custom|UpdateSpeed
  (bind _playermode (Variables|ModeInfo|GetPlayerMode))
  (bind _charactermovement (Variables|Character|GetCharacterMovement))
  (if (Utilities|Enum|Equal(Enum) _playermode "NewEnumerator2")
    (if (Variables|Movement|GetIsSprinting)
      (Variables|/Script/Engine.CharacterMovementComponent|SetMaxWalkSpeed _charactermovement (Variables|Movement|GetSprintSpeed))
      (else
        (Variables|/Script/Engine.CharacterMovementComponent|SetMaxWalkSpeed _charactermovement (Variables|Movement|GetWalkSpeed))))
    (elif (Utilities|Enum|Equal(Enum) _playermode "NewEnumerator0")
      (Variables|/Script/Engine.CharacterMovementComponent|SetMaxWalkSpeed _charactermovement 0.0))))

(event Custom|StopCrouch
  ;[1 1 1] Handles crouching
  (if (Utilities|Enum|Equal(Enum) (Variables|ModeInfo|GetPlayerMode) "NewEnumerator2")
    (Character|UnCrouch)))

(event Custom|StartSprinting
  ;[1 1 1] Handles Sprinting
  (if (Utilities|Enum|Equal(Enum) (Variables|ModeInfo|GetPlayerMode) "NewEnumerator2")
    (Variables|Movement|SetIsSprinting true)))

(event Custom|StopSprinting
  ;[1 1 1] Handles Sprinting
  (if (Utilities|Enum|Equal(Enum) (Variables|ModeInfo|GetPlayerMode) "NewEnumerator2")
    (Variables|Movement|SetIsSprinting false)))

(event Custom|CallJump
  ;[1 1 1] Handles Jumping
  (if (not (and false (Utilities|Enum|Equal(Enum) (Variables|ModeInfo|GetPlayerMode) "NewEnumerator2")))
    (Character|Jump)))

(event Custom|MoveRight
  (params (AxisValue :type Float%20%28double-precision%29))
  (bind _returnvalue (Transformation|GetActorRightVector))
  (bind _returnvalue_2 (Transformation|GetActorLocation))
  (bind _returnvalue_3 (Transformation|GetActorRightVector))
  (bind _oversightspeed (Variables|Oversight|GetOversightSpeed))
  (bind _returnvalue_4 (* _returnvalue_3 AxisValue))
  (bind _returnvalue_5 (* _returnvalue AxisValue))
  (bind _returnvalue_6 (* _returnvalue_5 _oversightspeed))
  (bind _returnvalue_7 (+ (Math|Vector|MakeVector (.x _returnvalue_2) (.y _returnvalue_2) (.z _returnvalue_2)) _returnvalue_6))
  ;[1 1 1] Handles Movement Logic
  (switch Utilities|FlowControl|Switch|SwitchonCharacterMode (Variables|ModeInfo|GetPlayerMode)
    (:NewEnumerator0
      (bind _out (CallFunction|LocktoBounds (Math|Vector|MakeVector (.x _returnvalue_7) (.y _returnvalue_7) (.z _returnvalue_2))))
      (Transformation|SetActorLocation _out false false)
      (CallFunction|UpdateActorLocation _out))
    (:NewEnumerator2
      (Pawn|Input|AddMovementInput (Math|Vector|MakeVector (.x _returnvalue_4) (.y _returnvalue_4) 0.0) 1.0 false))))

(event Custom|MoveForward
  (params (AxisValue :type Float%20%28double-precision%29))
  (bind _returnvalue (Transformation|GetActorLocation))
  (bind _returnvalue_2 (Transformation|GetActorForwardVector))
  (bind _returnvalue_3 (Transformation|GetActorForwardVector))
  (bind _oversightspeed (Variables|Oversight|GetOversightSpeed))
  (bind _returnvalue_4 (* _returnvalue_3 AxisValue))
  (bind _returnvalue_5 (* _returnvalue_2 AxisValue))
  (bind _returnvalue_6 (* _returnvalue_4 _oversightspeed))
  (bind _returnvalue_7 (+ (Math|Vector|MakeVector (.x _returnvalue) (.y _returnvalue) (.z _returnvalue)) _returnvalue_6))
  ;[1 1 1] Handles Movement Logic
  (switch Utilities|FlowControl|Switch|SwitchonCharacterMode (Variables|ModeInfo|GetPlayerMode)
    (:NewEnumerator0
      (bind _out (CallFunction|LocktoBounds (Math|Vector|MakeVector (.x _returnvalue_7) (.y _returnvalue_7) (.z _returnvalue))))
      (Transformation|SetActorLocation _out false false)
      (CallFunction|UpdateActorLocation _out))
    (:NewEnumerator2
      (Pawn|Input|AddMovementInput (Math|Vector|MakeVector (.x _returnvalue_5) (.y _returnvalue_5) 0.0) 1.0 false))))

(event Custom|SetOversightBounds
  (params (X :type Float%20%28double-precision%29) (Y :type Float%20%28double-precision%29))
  (Variables|Oversight|SetOversightBoundX X)
  (Variables|Oversight|SetOversightBoundY Y))

(event Input|EnhancedActionEvents|EnhancedInputActionIA_Jump
  (params (ActionValue :type Boolean) (ElapsedSeconds :type Float%20%28double-precision%29) (TriggeredSeconds :type Float%20%28double-precision%29) (InputAction :type Input%20Action%20Object%20Reference :default "/Game/Input/InputActions/IA_Jump.IA_Jump"))
  ;[1 1 1] Handles Jumping
  (CallFunction|CallJump))

(event Input|EnhancedActionEvents|EnhancedInputActionIA_ToggleMode
  (params (ActionValue :type Boolean) (ElapsedSeconds :type Float%20%28double-precision%29) (TriggeredSeconds :type Float%20%28double-precision%29) (InputAction :type Input%20Action%20Object%20Reference :default "/Game/Input/InputActions/IA_ToggleMode.IA_ToggleMode"))
  (bind _playermode (Variables|ModeInfo|GetPlayerMode))
  (if (or (Utilities|Enum|Equal(Enum) _playermode "NewEnumerator0") (Utilities|Enum|Equal(Enum) _playermode "NewEnumerator2"))
    (CallFunction|ToggleMode)))

(event Input|EnhancedActionEvents|EnhancedInputActionIA_BeginSprint
  (params (ActionValue :type Boolean) (ElapsedSeconds :type Float%20%28double-precision%29) (TriggeredSeconds :type Float%20%28double-precision%29) (InputAction :type Input%20Action%20Object%20Reference :default "/Game/Input/InputActions/IA_BeginSprint.IA_BeginSprint"))
  ;[1 1 1] Handles Sprinting
  (CallFunction|StartSprinting))

(event Input|EnhancedActionEvents|EnhancedInputActionIA_Look
  (params (ActionValue :type Vector%202D%20Structure) (ElapsedSeconds :type Float%20%28double-precision%29) (TriggeredSeconds :type Float%20%28double-precision%29) (InputAction :type Input%20Action%20Object%20Reference :default "/Game/Input/InputActions/IA_Look.IA_Look"))
  (bind (_x _y) (Math|Vector2D|BreakVector2D ActionValue))
  ;[1 1 1] Looking
  (Pawn|Input|AddControllerPitchInput (* _y -1.0))
  (Pawn|Input|AddControllerYawInput _x))

(event Input|EnhancedActionEvents|EnhancedInputActionIA_EndSprint
  (params (ActionValue :type Boolean) (ElapsedSeconds :type Float%20%28double-precision%29) (TriggeredSeconds :type Float%20%28double-precision%29) (InputAction :type Input%20Action%20Object%20Reference :default "/Game/Input/InputActions/IA_EndSprint.IA_EndSprint"))
  ;[1 1 1] Handles Sprinting
  (CallFunction|StopSprinting))

(event Input|EnhancedActionEvents|EnhancedInputActionIA_BeginCrouch
  (params (ActionValue :type Boolean) (ElapsedSeconds :type Float%20%28double-precision%29) (TriggeredSeconds :type Float%20%28double-precision%29) (InputAction :type Input%20Action%20Object%20Reference :default "/Game/Input/InputActions/IA_BeginCrouch.IA_BeginCrouch"))
  ;[1 1 1] Handles crouching
  (CallFunction|StartCrouch))

(event Input|EnhancedActionEvents|EnhancedInputActionIA_Move
  (params (ActionValue :type Vector%202D%20Structure) (ElapsedSeconds :type Float%20%28double-precision%29) (TriggeredSeconds :type Float%20%28double-precision%29) (InputAction :type Input%20Action%20Object%20Reference :default "/Game/Input/InputActions/IA_Move.IA_Move"))
  (bind (_x _y) (Math|Vector2D|BreakVector2D ActionValue))
  (bind _playermode (Variables|ModeInfo|GetPlayerMode))
  ;[1 1 1] Also Movement Logic
  (if (or (Utilities|Enum|Equal(Enum) _playermode "NewEnumerator0") (Utilities|Enum|Equal(Enum) _playermode "NewEnumerator2"))
    (CallFunction|MoveRight _x)
    (CallFunction|MoveForward _y)))

(event Input|EnhancedActionEvents|EnhancedInputActionIA_EndCrouch
  (params (ActionValue :type Boolean) (ElapsedSeconds :type Float%20%28double-precision%29) (TriggeredSeconds :type Float%20%28double-precision%29) (InputAction :type Input%20Action%20Object%20Reference :default "/Game/Input/InputActions/IA_EndCrouch.IA_EndCrouch"))
  ;[1 1 1] Handles crouching
  (CallFunction|StopCrouch))

(event EventTick
  (params (DeltaSeconds :type Float%20%28single-precision%29))
  (bind _charactermovement (Variables|Character|GetCharacterMovement))
  (Utilities|FlowControl|Sequence
    (:then_0
      ;[1 1 1] Controls Gravity Scale
      (if (Utilities|Enum|Equal(Enum) (Variables|ModeInfo|GetPlayerMode) "NewEnumerator2")
        (Variables|/Script/Engine.CharacterMovementComponent|SetGravityScale _charactermovement (Variables|Movement|GetDefaultGravityScale))
        (elif (Utilities|Enum|Equal(Enum) (Variables|ModeInfo|GetPlayerMode) "NewEnumerator1")
          (Variables|/Script/Engine.CharacterMovementComponent|SetGravityScale _charactermovement (Variables|Movement|GetFallingGravityScale))
          (else
            (Variables|/Script/Engine.CharacterMovementComponent|SetGravityScale _charactermovement 0.0)))))
    (:then_1
      (switch Utilities|FlowControl|Switch|SwitchonCharacterMode (Variables|ModeInfo|GetPlayerMode)
        (:NewEnumerator0
          (Variables|/Script/Engine.MovementComponent|SetVelocity (Variables|Character|GetCharacterMovement) "0, 0, 0"))
        (:NewEnumerator1
          (if (AI|Components|NavMovement|IsMovingonGround (Variables|Character|GetCharacterMovement))
            (Variables|ModeInfo|SetPlayerMode "NewEnumerator2")
            (Variables|Movement|SetIsSprinting false)))
        (:NewEnumerator3
          (if (>= (.z (Transformation|GetActorLocation)) (Variables|Oversight|GetOversightAscendTo))
            (Variables|ModeInfo|SetPlayerMode "NewEnumerator0")
            (Variables|Movement|SetIsSprinting false)
            (else
              (Networking|SwitchHasAuthority
                (:Authority
                  (CallFunction|RisetoOversight DeltaSeconds))))))))))

(event EventBeginPlay
  ;[1 1 1] Begin Play - Set Terminal Velocity
  (bind _outactors (Actor|GetAllActorsOfClass "/Script/Engine.PhysicsVolume"))
  (for _array_element _outactors
    (Variables|/Script/Engine.PhysicsVolume|SetTerminalVelocity _array_element (Variables|Movement|GetTerminalVelocity))))

(fn ConstructionScript)

(fn SetFOV
  (params (Target :type Float%20%28double-precision%29))
  (Camera|SetFieldOfView (Variables|Default|GetCamera) (Math|Interpolation|FInterpTo (Variables|/Script/Engine.CameraComponent|GetFieldOfView (Variables|Default|GetCamera)) Target (Utilities|Time|GetWorldDeltaSeconds) (Variables|CameraSettings|GetFOVInterpolationSpeed))))

(fn SetFOVPerTick
  (switch int 0
    (:0
      (CallFunction|SetFOV (select false (Variables|CameraSettings|GetSprintingFOV) (Variables|CameraSettings|GetDefaultFOV)) :!label _label))
    (:1
      (goto _label))
    (:2
      (CallFunction|SetFOV (Variables|CameraSettings|GetPlayerModeTransitionFOV) :!label _label_2))
    (:3
      (goto _label_2))))

(fn UpdateCameraShake
  (bind _returnvalue (Game|GetPlayerController 0))
  (switch int 0
    (:0
      (if true
        (Game|Feedback|ClientStartCameraShake _returnvalue "/Game/HeadBob/Sprint.Sprint_C" 0.25 "CameraLocal" "0, 0, 0")
        (elif (<= (Math|Vector|VectorLength (Transformation|GetVelocity)) 0.0)
          (Game|Feedback|ClientStartCameraShake _returnvalue "/Game/HeadBob/Idle.Idle_C" 0.25 "CameraLocal" "0, 0, 0")
          (else
            (Game|Feedback|ClientStartCameraShake _returnvalue "/Game/HeadBob/Walk.Walk_C" 0.25 "CameraLocal" "0, 0, 0")))))
    (:1
      (Game|Feedback|ClientStartCameraShake _returnvalue "/Game/HeadBob/Airborne.Airborne_C" 0.25 "CameraLocal" "0, 0, 0" :!label _label))
    (:2
      (goto _label))
    (:3
      (goto _label))))

(fn SetMeshVisibility
  (bind _mesh (Variables|Character|GetMesh))
  (switch int 0
    (:0
      (if (AI|Components|NavMovement|IsFalling (Variables|Character|GetCharacterMovement))
        (Class|PrimitiveComponent|SetOwnerNoSee _mesh false :!label _label)
        (else
          (Class|PrimitiveComponent|SetOwnerNoSee _mesh true))))
    (:1
      (goto _label))
    (:2
      (goto _label))
    (:3
      (goto _label))))

(fn LocktoBounds
  (params (In :type Vector))
  (bind _oversightboundy (Variables|Oversight|GetOversightBoundY))
  (bind _oversightboundx (Variables|Oversight|GetOversightBoundX))
  (bind _oversightboundy_2 (Variables|Oversight|GetOversightBoundY))
  (bind _oversightboundx_2 (Variables|Oversight|GetOversightBoundX))
  (bind _returnvalue (* _oversightboundx_2 -1.0))
  (bind _returnvalue_2 (* _oversightboundy -1.0))
  (LocalVariables|SetLockedVector In)
  (Utilities|FlowControl|Sequence
    (:then_0
      (if (< (.x (LocalVariables|GetLockedVector)) _returnvalue)
        (LocalVariables|SetLockedVector (Math|Vector|MakeVector _returnvalue (.y (LocalVariables|GetLockedVector)) (.z (LocalVariables|GetLockedVector))))))
    (:then_1
      (if (< (.y (LocalVariables|GetLockedVector)) _returnvalue_2)
        (LocalVariables|SetLockedVector (Math|Vector|MakeVector (.x (LocalVariables|GetLockedVector)) _returnvalue_2 (.z (LocalVariables|GetLockedVector))))))
    (:then_2
      (if (> (.x (LocalVariables|GetLockedVector)) _oversightboundx)
        (LocalVariables|SetLockedVector (Math|Vector|MakeVector _oversightboundx (.y (LocalVariables|GetLockedVector)) (.z (LocalVariables|GetLockedVector))))))
    (:then_3
      (if (> (.y (LocalVariables|GetLockedVector)) _oversightboundy_2)
        (LocalVariables|SetLockedVector (Math|Vector|MakeVector (.x (LocalVariables|GetLockedVector)) _oversightboundy_2 (.z (LocalVariables|GetLockedVector))))))
    (:then_4
      (return (LocalVariables|GetLockedVector)))))

(fn OnRepIsSprinting
  (CallFunction|UpdateSpeed))