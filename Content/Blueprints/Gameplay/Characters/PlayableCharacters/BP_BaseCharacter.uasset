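; Base playable character that forwards Enhanced Input for movement, look, jump, crouch, sprint and mode toggling to movement and state functions.
; Tick drives interpolated FOV, camera shake and owner-only mesh hiding from player mode, sprint, velocity and falling state.
; Autoattack spawns a cooldown-gated projectile ahead of the right hand and returns its cost when fired.
; SetPlayerInitPosition places the character by selection index using the BP_GridManager found on BeginPlay.
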(event Input|EnhancedActionEvents|EnhancedInputActionIA_Jump
  (params (ActionValue :type Boolean) (ElapsedSeconds :type Float%20%28double-precision%29) (TriggeredSeconds :type Float%20%28double-precision%29) (InputAction :type Input%20Action%20Object%20Reference :default "/Game/Input/InputActions/IA_Jump.IA_Jump"))
  (Class|MyCharacter|CallJump))

(event Input|EnhancedActionEvents|EnhancedInputActionIA_BeginSprint
  (params (ActionValue :type Boolean) (ElapsedSeconds :type Float%20%28double-precision%29) (TriggeredSeconds :type Float%20%28double-precision%29) (InputAction :type Input%20Action%20Object%20Reference :default "/Game/Input/InputActions/IA_BeginSprint.IA_BeginSprint"))
  (Class|MyCharacter|StartSprint))

(event Input|EnhancedActionEvents|EnhancedInputActionIA_Look
  (params (ActionValue :type Vector%202D%20Structure) (ElapsedSeconds :type Float%20%28double-precision%29) (TriggeredSeconds :type Float%20%28double-precision%29) (InputAction :type Input%20Action%20Object%20Reference :default "/Game/Input/InputActions/IA_Look.IA_Look"))
  (bind (_x _y) (Math|Vector2D|BreakVector2D ActionValue))
  (Pawn|Input|AddControllerPitchInput (* _y -1.0))
  (Pawn|Input|AddControllerYawInput _x))

(event Input|EnhancedActionEvents|EnhancedInputActionIA_EndSprint
  (params (ActionValue :type Boolean) (ElapsedSeconds :type Float%20%28double-precision%29) (TriggeredSeconds :type Float%20%28double-precision%29) (InputAction :type Input%20Action%20Object%20Reference :default "/Game/Input/InputActions/IA_EndSprint.IA_EndSprint"))
  (Class|MyCharacter|StopSprint))

(event Input|EnhancedActionEvents|EnhancedInputActionIA_BeginCrouch
  (params (ActionValue :type Boolean) (ElapsedSeconds :type Float%20%28double-precision%29) (TriggeredSeconds :type Float%20%28double-precision%29) (InputAction :type Input%20Action%20Object%20Reference :default "/Game/Input/InputActions/IA_BeginCrouch.IA_BeginCrouch"))
  (Character|Crouch)
  (Class|MyCharacter|StartCrouch))

(event Input|EnhancedActionEvents|EnhancedInputActionIA_ToggleMode
  (params (ActionValue :type Boolean) (ElapsedSeconds :type Float%20%28double-precision%29) (TriggeredSeconds :type Float%20%28double-precision%29) (InputAction :type Input%20Action%20Object%20Reference :default "/Game/Input/InputActions/IA_ToggleMode.IA_ToggleMode"))
  (Class|MyCharacter|ToggleMode)
  (Class|MyCharacter|GetPlayerMode))

(event Input|EnhancedActionEvents|EnhancedInputActionIA_Move
  (params (ActionValue :type Vector%202D%20Structure) (ElapsedSeconds :type Float%20%28double-precision%29) (TriggeredSeconds :type Float%20%28double-precision%29) (InputAction :type Input%20Action%20Object%20Reference :default "/Game/Input/InputActions/IA_Move.IA_Move"))
  (bind (_x _y) (Math|Vector2D|BreakVector2D ActionValue))
  (Class|MyCharacter|MoveRight _x)
  (Class|MyCharacter|MoveForward _y))

(event Input|EnhancedActionEvents|EnhancedInputActionIA_EndCrouch
  (params (ActionValue :type Boolean) (ElapsedSeconds :type Float%20%28double-precision%29) (TriggeredSeconds :type Float%20%28double-precision%29) (InputAction :type Input%20Action%20Object%20Reference :default "/Game/Input/InputActions/IA_EndCrouch.IA_EndCrouch"))
  (Character|UnCrouch)
  (Class|MyCharacter|StopCrouch))

(event EventBeginPlay
  (bind _returnvalue (Actor|GetActorOfClass "/Game/Blueprints/Gameplay/Managers/BP_GridManager.BP_GridManager_C"))
  (Variables|Default|SetGridManager _returnvalue))

(event Collision|EventActorBeginOverlap
  (params (OtherActor :type Actor%20Object%20Reference)))

(event EventTick
  (params (DeltaSeconds :type Float%20%28single-precision%29))
  (CallFunction|SetFOVPerTick)
  (CallFunction|UpdateCameraShake)
  (CallFunction|SetMeshVisibility)
  (CallFunction|TickAutoattackCooldown DeltaSeconds))

(fn ConstructionScript)

(fn SetFOV
  (params (Target :type Float%20%28double-precision%29))
  (Camera|SetFieldOfView (Variables|Default|GetCamera) (Math|Interpolation|FInterpTo (Variables|/Script/Engine.CameraComponent|GetFieldOfView (Variables|Default|GetCamera)) Target (Utilities|Time|GetWorldDeltaSeconds) (Variables|Default|GetFOVInterpolationSpeed))))

(fn SetPlayerInitPosition
  (params (Selection :type Integer))
  (bind _returnvalue (Class|GridManager|GetPlayerSpawnPosition (Variables|Default|GetGridManager)))
  (switch int Selection
    (:0
      (Transformation|SetActorLocationAndRotation (Math|Vector|MakeVector (Math|Conversions|ToFloat(Integer) _returnvalue) (Math|Conversions|ToFloat(Integer) _returnvalue) 2.5e+02) "0.000000,45.000000,0.000000"))
    (:1
      (Transformation|SetActorLocationAndRotation (Math|Vector|MakeVector (Math|Conversions|ToFloat(Integer) _returnvalue) (Math|Conversions|ToFloat(Integer) (* _returnvalue -1)) 2.5e+02) "0.000000,90.000000,0.000000"))
    (:2
      (Transformation|SetActorLocationAndRotation (Math|Vector|MakeVector (Math|Conversions|ToFloat(Integer) (* _returnvalue -1)) (Math|Conversions|ToFloat(Integer) (* _returnvalue -1)) 2.5e+02) "0.000000,180.000000,0.000000"))
    (:3
      (Transformation|SetActorLocationAndRotation (Math|Vector|MakeVector (Math|Conversions|ToFloat(Integer) (* _returnvalue -1)) (Math|Conversions|ToFloat(Integer) (* _returnvalue -1)) 2.5e+02) "0, 0, 0"))))

(fn SetFOVPerTick
  (bind _returnvalue (Class|MyCharacter|GetPlayerMode))
  (switch int _returnvalue
    (:0
      (bind _returnvalue_2 (Class|MyCharacter|GetIsSprinting :!label _label))
      (CallFunction|SetFOV (select _returnvalue_2 (Variables|Default|GetSprintingFOV) (Variables|Default|GetDefaultFOV))))
    (:1
      (goto _label))
    (:2
      (CallFunction|SetFOV (Variables|Default|GetPlayerModeTransitionFOV) :!label _label_2))
    (:3
      (goto _label_2))))

(fn UpdateCameraShake
  (bind _returnvalue (Game|GetPlayerController 0))
  (bind _returnvalue_2 (Class|MyCharacter|GetPlayerMode))
  (switch int _returnvalue_2
    (:0
      (bind _returnvalue_3 (Class|MyCharacter|GetIsSprinting))
      (if _returnvalue_3
        (Game|Feedback|ClientStartCameraShake _returnvalue "/Game/HeadBob/Sprint.Sprint_C" 0.25 "CameraLocal" "0, 0, 0")
        (elif (<= (Math|Vector|VectorLength (Transformation|GetVelocity)) 0.0)
          (Game|Feedback|ClientStartCameraShake _returnvalue "/Game/HeadBob/Idle.Idle_C" 0.25 "CameraLocal" "0, 0, 0")
          (else
            (Game|Feedback|ClientStartCameraShake _returnvalue "/Game/HeadBob/Walk.Walk_C" 0.25 "CameraLocal" "0, 0, 0")))))
    (:1
      (Game|Feedback|ClientStartCameraShake _returnvalue "/Game/HeadBob/Airborne.Airborne_C" 0.25 "CameraLocal" "0, 0, 0" :!label _label))
    (:2
      (goto _label))
    (:3
      (goto _label))))

(fn SetMeshVisibility
  (bind _mesh (Variables|Character|GetMesh))
  (bind _returnvalue (Class|MyCharacter|GetPlayerMode))
  (switch int _returnvalue
    (:0
      (if (AI|Components|NavMovement|IsFalling (Variables|Character|GetCharacterMovement))
        (Class|PrimitiveComponent|SetOwnerNoSee _mesh false :!label _label)
        (else
          (Class|PrimitiveComponent|SetOwnerNoSee _mesh true))))
    (:1
      (goto _label))
    (:2
      (goto _label))
    (:3
      (goto _label))))

(fn Autoattack
  (if (<= (Variables|Default|GetCurrentAutoattackCooldownTimer) 0.0)
    (Game|SpawnActorfromClass (Variables|Default|GetAutoattackProjectile) (Math|Transform|MakeTransform (+ (Transformation|GetSocketLocation (Variables|Default|GetSkeletalMesh) "hand_r") (* (Transformation|GetActorForwardVector) "1000.000000,1000.000000,1000.000000")) (Transformation|GetActorRotation) "1.000000,1.000000,1.000000") "Undefined" "MultiplyWithRoot" 0 0)
    (Variables|Default|SetCurrentAutoattackCooldownTimer (Variables|Default|GetAutoattackCooldown))
    (return (Variables|Default|GetAutoattackCost))))

(fn TickAutoattackCooldown
  (params (B :type Float%20%28double-precision%29))
  (Variables|Default|SetCurrentAutoattackCooldownTimer (- (Variables|Default|GetCurrentAutoattackCooldownTimer) B)))