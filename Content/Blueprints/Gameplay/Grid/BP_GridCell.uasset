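; BP_GridCell is a grid cell actor whose cube mesh displays a replicated base color.
; SetColor writes the BaseColor variable, whose RepNotify calls UpdateColor.
; UpdateColor lazily creates and caches a dynamic material instance on the cube, then sets its BaseColor vector parameter.
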(event Custom|SetColor
  (params (Color :type Vector))
  (Variables|Default|SetBaseColor Color))

(event Custom|UpdateColor
  (bind _cube (Variables|Default|GetCube))
  (Utilities|IsValid (Variables|Default|GetCellMaterial)
    (:Is%20Valid
      _)
    (:Is%20Not%20Valid
      (bind _returnvalue (Rendering|Material|CreateDynamicMaterialInstance _cube 0 (Rendering|Material|GetMaterial _cube 0) "None" :!class /Script/Engine.PrimitiveComponent))
      (Rendering|Material|SetMaterial _cube 0 _returnvalue)
      (bind _output_get (Variables|Default|SetCellMaterial _returnvalue))))
  (Rendering|Material|SetVectorParameterValue _output_get "BaseColor" (Math|Conversions|ToLinearColor(Vector) (Variables|Default|GetBaseColor)) :!class /Script/Engine.MaterialInstanceDynamic))

(fn ConstructionScript)

(fn OnRepBaseColor
  (CallFunction|UpdateColor))