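; Base neutral camp inhabitant that tracks health and periodically attacks nearby characters.
; Tick turns its info widget toward the camera and feeds it health values, while debug-printing the attack cooldown.
; On authority, a sphere overlap damages one BP_BaseCharacter in range whenever the cooldown expires.
; Player controller 0 relays cooldown updates and, when AlterHealth depletes health, notifies the game mode of the death and slayer.
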(event Custom|AlterHealth
  (params (Amount :type Float%20%28double-precision%29) (HitByPlayerId :type Integer))
  (bind _output_get (Variables|Default|SetHealth (+ (Variables|Default|GetHealth) Amount)))
  (if (<= _output_get 0.0)
    (bind _asbp_my_player_controller (Utilities|Casting|CastToBP_MyPlayerController (Class|GameplayStatics|GetPlayerControllerfromID)))
    (Default|NotifyGameModeOfNeutralCampDeath _asbp_my_player_controller HitByPlayerId self)))

(event EventBeginPlay
  (Variables|Default|SetHealth (Variables|Default|GetMaxHealth)))

(event Collision|EventActorBeginOverlap
  (params (OtherActor :type Actor%20Object%20Reference)))

(event EventTick
  (params (DeltaSeconds :type Float%20%28single-precision%29))
  (bind _neutralinfowidget (Variables|Default|GetNeutralInfoWidget))
  (Development|PrintString (Utilities|String|ToString(Float) (Variables|Default|GetAttackCdTimer)))
  (Transformation|SetWorldRotation _neutralinfowidget (Math|Rotator|FindLookatRotation (Transformation|GetWorldLocation _neutralinfowidget) (Transformation|GetWorldLocation (Variables|/Script/Engine.Actor|GetRootComponent (Game|GetPlayerCameraManager 0)))) false false)
  (bind _aswbp_neutral_ui (Utilities|Casting|CastToWBP_NeutralUI (UserInterface|GetWidget (Variables|Default|GetNeutralInfoWidget))))
  (Variables|/Game/Blueprints/UI/Units/WBP_NeutralUI.WBP_NeutralUI_C|SetCurHealth _aswbp_neutral_ui (Variables|Default|GetHealth))
  (Variables|/Game/Blueprints/UI/Units/WBP_NeutralUI.WBP_NeutralUI_C|SetMaxHealth _aswbp_neutral_ui (Variables|Default|GetMaxHealth))
  (Networking|SwitchHasAuthority
    (:Authority
      (if (<= (Variables|Default|GetAttackCdTimer) 0.0)
        (bind _outactors (Collision|SphereOverlapActors (Transformation|GetActorLocation) (Variables|Default|GetAttackRange) (Utilities|Array|MakeArray "ObjectTypeQuery1" "ObjectTypeQuery2" "ObjectTypeQuery3") "/Game/Blueprints/Gameplay/Characters/BP_BaseCharacter.BP_BaseCharacter_C"))
        (bind _array_element (Utilities|Array|ForEachLoopwithBreak _outactors :!label _label)
          (:LoopBody
            (bind _asbp_base_character (Utilities|Casting|CastToBP_BaseCharacter _array_element))
            (Utilities|IsValid _asbp_base_character
              (:Is%20Valid
                (Default|AlterHP _asbp_base_character (* (Variables|Default|GetAttackDamage) -1.0))
                (Variables|Default|SetAttackCdTimer (Variables|Default|GetTimeBetweenAttacks))
                (bind _asbp_my_player_controller (Utilities|Casting|CastToBP_MyPlayerController (Class|GameplayStatics|GetPlayerControllerfromID)))
                (Utilities|IsValid _asbp_my_player_controller
                  (:Is%20Valid
                    (Default|SSetNeutralAttackCd _asbp_my_player_controller self (Variables|Default|GetTimeBetweenAttacks))
                    (goto _label Break)))))))
        (else
          (Variables|Default|SetAttackCdTimer (- (Variables|Default|GetAttackCdTimer) (Utilities|Time|GetWorldDeltaSeconds)))
          (bind _asbp_my_player_controller_2 (Utilities|Casting|CastToBP_MyPlayerController (Class|GameplayStatics|GetPlayerControllerfromID)))
          (Utilities|IsValid _asbp_my_player_controller_2
            (:Is%20Valid
              (Default|SSetNeutralAttackCd _asbp_my_player_controller_2 self (Variables|Default|GetAttackCdTimer)))))))))

(fn ConstructionScript)