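; Base combat unit with health, shield, resource, up to three stat-modifying items and active traits.
; A replicated InCombat flag resets vitals on entering or leaving combat, with entry granting a trait-ranked shield and combat ticks regenerating resource.
; Damage drains shield before health, with death reported to the game mode by owning player.
; Tick feeds a camera-facing widget with stats, tier and items; attack and ability are print-only placeholders.
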(event Custom|AlterHP
  (params (Amount :type Float%20%28double-precision%29))
  (if (Variables|Default|GetAlive)
    (if (> Amount 0.0)
      (Variables|Default|SetCurrentHealth (+ Amount (Variables|Default|GetCurrentHealth)))
      (elif (< Amount 0.0)
        (if (> (Variables|Default|GetCurrentShield) 0.0)
          (if (> (Math|Float|Absolute(Float) Amount) (Variables|Default|GetCurrentShield))
            (Variables|Default|SetCurrentHealth (+ (+ (Variables|Default|GetCurrentShield) Amount) (Variables|Default|GetCurrentShield)))
            (Variables|Default|SetCurrentShield 0.0)
            (else
              (Variables|Default|SetCurrentShield (+ (Variables|Default|GetCurrentShield) Amount))))
          (else
            (bind _output_get (Variables|Default|SetCurrentHealth (+ Amount (Variables|Default|GetCurrentHealth))))
            (if (and (Variables|Default|GetAlive) (<= _output_get 0.0))
              (Variables|Default|SetAlive false)
              (CallFunction|SNotifyGameModeOfDeath))))))))

(event Custom|SetItemUI
  (params (Items :type Array%20of%20BP%20Unit%20Item%20Base%20Object%20References))
  (bind _unitui (Variables|Widgets|GetUnitUI))
  (for _index (range 0 2)
    (if (>= _index (Utilities|Array|Length Items))
      (Default|SetItemVisibility _unitui _index "Hidden")
      (else
        (Default|SetItemVisibility _unitui _index "Visible")
        (bind _newparam (Default|GetItemImage _unitui _index))
        (Class|Image|SetBrush _newparam (Utilities|Struct|MakeSlateBrush "Image" "NoTile" "NoMirror" "(X=32.000000,Y=32.000000)" "(Left=0.000000,Top=0.000000,Right=0.000000,Bottom=0.000000)" "(SpecifiedColor=(R=1.000000,G=1.000000,B=1.000000,A=1.000000),ColorUseRule=UseColor_Specified)" "(CornerRadii=(X=0.000000,Y=0.000000,Z=0.000000,W=1.000000),Color=(SpecifiedColor=(R=0.000000,G=0.000000,B=0.000000,A=0.000000),ColorUseRule=UseColor_Specified),Width=0.000000,RoundingType=HalfHeightRadius,bUseBrushTransparency=False)" (Variables|/Game/Blueprints/Gameplay/Items/BP_UnitItemBase.BP_UnitItemBase_C|GetImage (Utilities|Array|Get(acopy) Items _index))))))))

(event Custom|TakeOffensiveAction
  (if (>= (Variables|Default|GetCurrentResource) 1e+02)
    (Development|PrintString "Cast Ability")
    (Variables|Default|SetCurrentResource 0.0)
    (else
      (Development|PrintString "Attack"))))

(event Custom|S_NotifyGameModeOfDeath
  (bind _asbp_my_game_mode (Utilities|Casting|CastToBP_MyGameMode (Game|GetGameMode)))
  (Utilities|IsValid _asbp_my_game_mode
    (:Is%20Valid
      (Default|SUnitDied _asbp_my_game_mode (Variables|Default|GetOwnedByPlayerID)))))

(event Custom|ApplyItemStats
  (params (Item :type Unit%20Item%20Stats%20Structure) (Multiplier :type Integer))
  (Variables|Stats|SetMaxHealth (+ (Variables|Stats|GetMaxHealth) (* (.maxhealth Item) Multiplier)))
  (Variables|Stats|SetMaxResource (+ (* (.maxresource Item) Multiplier) (Variables|Stats|GetMaxResource)))
  (Variables|Stats|SetAttackDamage (+ (* (.attackdamage Item) Multiplier) (Variables|Stats|GetAttackDamage)))
  (Variables|Stats|SetArmor (+ (* (.armor Item) Multiplier) (Variables|Stats|GetArmor)))
  (Variables|Stats|SetMoveSpeed (+ (* (.movespeed Item) Multiplier) (Variables|Stats|GetMoveSpeed)))
  (Variables|Stats|SetAttacksPerSecond (+ (* (.attackspersecond Item) Multiplier) (Variables|Stats|GetAttacksPerSecond)))
  (CallFunction|PrintStats))

(event Custom|UnequipItem
  (params (Item :type BP%20Unit%20Item%20Base%20Object%20Reference))
  (CallFunction|ApplyItemStats (Variables|/Game/Blueprints/Gameplay/Items/BP_UnitItemBase.BP_UnitItemBase_C|GetStats Item) -1)
  (Utilities|Array|RemoveItem (Variables|Default|GetItemsEquipped) Item))

(event Custom|EquipItem
  (params (Item :type BP%20Unit%20Item%20Base%20Object%20Reference))
  (if (< (Utilities|Array|Length (Variables|Default|GetItemsEquipped)) 3)
    (CallFunction|ApplyItemStats (Variables|/Game/Blueprints/Gameplay/Items/BP_UnitItemBase.BP_UnitItemBase_C|GetStats Item) 1)
    (Utilities|Array|Add (Variables|Default|GetItemsEquipped) Item)))

(event Custom|OnExitCombat
  (Variables|Default|SetCurrentHealth (Variables|Stats|GetMaxHealth))
  (Variables|Default|SetCurrentResource 0.0))

(event Custom|OnEnterCombat
  (Variables|Default|SetAlive true)
  (Variables|Default|SetCurrentHealth (Variables|Stats|GetMaxHealth))
  (CallFunction|CheckEarthBonus))

(event EventBeginPlay
  (|CallParentFunction)
  (CallFunction|OnExitCombat))

(event EventTick
  (params (DeltaSeconds :type Float%20%28single-precision%29))
  (CallFunction|UpdateUnitUI)
  (CallFunction|SetItemUI (Variables|Default|GetItemsEquipped))
  (if (Variables|Default|GetInCombat)
    (if (< (Variables|Default|GetCurrentResource) (Variables|Stats|GetMaxResource))
      (Variables|Default|SetCurrentResource (+ (Variables|Default|GetCurrentResource) (Variables|Default|GetPassiveResourceRegenRate))))))

(fn ConstructionScript
  (|CallParentFunction))

(fn OnRepinCombat
  (if (Variables|Default|GetInCombat)
    (CallFunction|OnEnterCombat)
    (else
      (CallFunction|OnExitCombat))))

(fn PrintStats
  (Development|PrintString (Utilities|String|ToString(Text) (Utilities|Text|FormatText "MaxHealth: {MaxHealth}" (Variables|Stats|GetMaxHealth))))
  (Development|PrintString (Utilities|String|ToString(Text) (Utilities|Text|FormatText "MaxResource: {MaxResource}" (Variables|Stats|GetMaxResource))))
  (Development|PrintString (Utilities|String|ToString(Text) (Utilities|Text|FormatText "AttackDamage: {AttackDamage}" (Variables|Stats|GetAttackDamage))))
  (Development|PrintString (Utilities|String|ToString(Text) (Utilities|Text|FormatText "Armor: {Armor}" (Variables|Stats|GetArmor))))
  (Development|PrintString (Utilities|String|ToString(Text) (Utilities|Text|FormatText "Move Speed: {MoveSpeed}" (Variables|Stats|GetMoveSpeed))))
  (Development|PrintString (Utilities|String|ToString(Text) (Utilities|Text|FormatText "Attacks Per Second: {APS}" (Variables|Stats|GetAttacksPerSecond)))))

(fn UpdateUnitUI
  (bind _unitinfowidget (Variables|Default|GetUnitInfoWidget))
  (bind _returnvalue (UserInterface|GetWidget _unitinfowidget))
  (bind _aswbp_unit_ui (Utilities|Casting|CastToWBP_UnitUI _returnvalue))
  (Transformation|SetWorldRotation _unitinfowidget (Math|Rotator|FindLookatRotation (Transformation|GetWorldLocation (Variables|Default|GetUnitInfoWidget)) (Transformation|GetWorldLocation (Variables|/Script/Engine.Actor|GetRootComponent (Game|GetPlayerCameraManager 0)))) false false)
  (Variables|Widgets|SetUnitUI _aswbp_unit_ui)
  (Variables|/Game/Blueprints/UI/Units/WBP_UnitUI.WBP_UnitUI_C|SetCurHealth _aswbp_unit_ui (Variables|Default|GetCurrentHealth))
  (Variables|/Game/Blueprints/UI/Units/WBP_UnitUI.WBP_UnitUI_C|SetMaxHealth _aswbp_unit_ui (Variables|Stats|GetMaxHealth))
  (Variables|/Game/Blueprints/UI/Units/WBP_UnitUI.WBP_UnitUI_C|SetCurResource _aswbp_unit_ui (Variables|Default|GetCurrentResource))
  (Variables|/Game/Blueprints/UI/Units/WBP_UnitUI.WBP_UnitUI_C|SetMaxResource _aswbp_unit_ui (Variables|Stats|GetMaxResource))
  (Variables|/Game/Blueprints/UI/Units/WBP_UnitUI.WBP_UnitUI_C|SetCurShield _aswbp_unit_ui (Variables|Default|GetCurrentShield))
  (Rendering|Components|TextRender|SetText (Variables|/Game/Blueprints/UI/Units/WBP_UnitUI.WBP_UnitUI_C|GetLevel _aswbp_unit_ui) (Utilities|Text|ToText(Integer) (Variables|Default|GetTier))))

(fn GetTraitRank
  (params (Trait :type TraitType%20Enum :default "NewEnumerator0"))
  (for _array_element (Variables|Default|GetTraitMap)
    (if (Utilities|Enum|Equal(Enum) Trait (.Trait (Utilities|Struct|BreakTraitState _array_element)))
      (return (.NumActive (Utilities|Struct|BreakTraitState _array_element)))))
  (return 0))

(fn AddShield
  (params (Amount :type Float%20%28double-precision%29))
  (bind _output_get (Variables|Default|SetCurrentShield (Math|Float|Clamp(Float) (+ (Variables|Default|GetCurrentShield) Amount) 0.0 1e+02)))
  (Development|PrintString (Utilities|String|ToString(Float) _output_get)))

(fn CheckEarthBonus
  (Utilities|IsTraitActive "NewEnumerator3"
    (:True
      (bind _rank (CallFunction|GetTraitRank "NewEnumerator3"))
      (if (>= _rank 4)
        (CallFunction|AddShield 5e+01)
        (elif (>= _rank 3)
          (CallFunction|AddShield 2e+01)
          (elif (>= _rank 2)
            (CallFunction|AddShield 1e+01)))))))