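; BP_GoldVein is a minable gold vein with a hit count and a timed non-hittable state.
; On the authority, Tick counts down NonHittableTimer and refills HitsRemaining when it expires.
; Tick also turns the health widget toward the player camera and feeds it the remaining hits.
; The mesh swaps between hittable and non-hittable dynamic materials, created at BeginPlay, according to the timer.
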(event EventBeginPlay
  (bind _staticmesh (Variables|Default|GetStaticMesh))
  (|CallParentFunction)
  (bind _returnvalue (Rendering|Material|CreateDynamicMaterialInstance _staticmesh 0 "/Game/Blueprints/Gameplay/Units/Mat_GoldVeinNonHittable.Mat_GoldVeinNonHittable" "None" :!class /Script/Engine.PrimitiveComponent))
  (Variables|Default|SetNonHittableMatInstance _returnvalue)
  (bind _returnvalue_2 (Rendering|Material|CreateDynamicMaterialInstance _staticmesh 0 "/Game/Blueprints/Gameplay/Units/Mat_GoldVeinHittable.Mat_GoldVeinHittable" "None" :!class /Script/Engine.PrimitiveComponent))
  (Variables|Default|SetHittableMatInstance _returnvalue_2))

(event Collision|EventActorBeginOverlap
  (params (OtherActor :type Actor%20Object%20Reference)))

(event EventTick
  (params (DeltaSeconds :type Float%20%28single-precision%29))
  (bind _goldveinui (Variables|Default|GetGoldVeinUI))
  (bind _staticmesh (Variables|Default|GetStaticMesh))
  (Utilities|FlowControl|Sequence
    (:then_0
      (Transformation|SetWorldRotation _goldveinui (Math|Rotator|FindLookatRotation (Transformation|GetWorldLocation _goldveinui) (Transformation|GetWorldLocation (Variables|/Script/Engine.Actor|GetRootComponent (Game|GetPlayerCameraManager 0)))) false false)
      (bind _output_get (Variables|Default|SetGoldVeinUIWidget (.AsWBP%20Gold%20Vein%20UI (Utilities|Casting|CastToWBP_GoldVeinUI (UserInterface|GetWidget (Variables|Default|GetGoldVeinUI))))))
      (Variables|/Game/Blueprints/UI/Units/WBP_GoldVeinUI.WBP_GoldVeinUI_C|SetCurHealth _output_get (Math|Conversions|ToFloat(Integer) (Variables|Default|GetHitsRemaining)))
      (Variables|/Game/Blueprints/UI/Units/WBP_GoldVeinUI.WBP_GoldVeinUI_C|SetMaxHealth _output_get 1e+01))
    (:then_1
      (Networking|SwitchHasAuthority
        (:Authority
          (if (> (Variables|Default|GetNonHittableTimer) 0.0)
            (bind _output_get_2 (Variables|Default|SetNonHittableTimer (- (Variables|Default|GetNonHittableTimer) (Utilities|Time|GetWorldDeltaSeconds))))
            (if (<= _output_get_2 0.0)
              (Variables|Default|SetHitsRemaining 10))))))
    (:then_2
      (if (> (Variables|Default|GetNonHittableTimer) 0.0)
        (Rendering|Material|SetMaterial _staticmesh 0 (Variables|Default|GetNonHittableMatInstance))
        (else
          (Rendering|Material|SetMaterial _staticmesh 0 (Variables|Default|GetHittableMatInstance)))))))

(fn ConstructionScript
  (|CallParentFunction))