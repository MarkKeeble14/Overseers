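; BP_BaseUnit is a unit actor that sits on a grid cell and has a tier and a rarity.
; On BeginPlay and each tier-up, capped at tier 3, it finds its BP_GridCell with a vertical line trace and scales itself by tier relative to that cell's size, within clamped limits.
; GetValue derives the unit's worth from rarity, growing exponentially with tier.
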(event Custom|S_TierUp
  (if (< (Variables|UnitInfo|GetTier) 3)
    (Variables|UnitInfo|SetTier (+ (Variables|UnitInfo|GetTier) 1))
    (CallFunction|SetScaleBasedonTier)))

(event Custom|SetScaleBasedOnTier
  (bind _oncell (Variables|Default|GetOnCell))
  (bind _returnvalue (Transformation|GetActorScale3D _oncell))
  (CallFunction|SetonCell)
  (Utilities|IsValid _oncell
    (:Is%20Valid
      (Transformation|SetActorScale3D (Math|Conversions|ToVector(Float) (Math|Float|Clamp(Float) (/ (* (Variables|UnitInfo|GetTier) (.x _returnvalue)) 5.0) 3.0 (.x _returnvalue)))))))

(event EventBeginPlay
  (CallFunction|SetScaleBasedonTier))

(fn ConstructionScript)

(fn SetonCell
  (bind _returnvalue (Transformation|GetActorLocation))
  (bind (_outhits _returnvalue_2) (Collision|MultiLineTraceByChannel (+ _returnvalue "0.000000,0.000000,500.000000") (+ _returnvalue (* (Transformation|GetActorUpVector) -5e+04)) "TraceTypeQuery3" false 0 "None"))
  (if _returnvalue_2
    (bind _array_element (Utilities|Array|ForEachLoopwithBreak _outhits :!label _label)
      (:LoopBody
        (if (.bBlockingHit (Collision|BreakHitResult _array_element))
          (bind _asbp_grid_cell (Utilities|Casting|CastToBP_GridCell (.HitActor (Collision|BreakHitResult _array_element))))
          (Development|PrintString "Set Cell")
          (Variables|Default|SetOnCell _asbp_grid_cell)
          (goto _label Break))))))

(fn GetValue
  (return (Math|Float|Truncate (* (Math|Float|Power 3.0 (Math|Conversions|ToFloat(Integer) (- (Variables|UnitInfo|GetTier) 1))) (Variables|UnitInfo|GetRarity)))))