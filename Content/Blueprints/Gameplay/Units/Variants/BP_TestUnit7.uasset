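; BP_TestUnit7 is a test unit variant whose ability hits and burns combat units along a line toward its target.
; CastAbility picks damage and burn duration by Tier, with tier 3 sharing the default's strongest values.
; A multi-object line trace runs to the target's location with timed debug drawing.
; Each BP_CombatUnitBase hit gets AlterHP and its BurningTimer set, with no team check.
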(event EventBeginPlay
  (|CallParentFunction) ; This node is disabled and will not be called.\nDrag off pins to build functionality.
)

(event Collision|EventActorBeginOverlap
  (params (OtherActor :type Actor%20Object%20Reference)))

(event EventTick
  (params (DeltaSeconds :type Float%20%28single-precision%29))
  (|CallParentFunction DeltaSeconds) ; This node is disabled and will not be called.\nDrag off pins to build functionality.
)

(event EventCastAbility
  (params (TargetingUnit :type BP%20Combat%20Unit%20Base%20Object%20Reference))
  (switch int (Variables|Default|GetTier)
    (:Default
      (Variables|Default|SetBurnDuration 5.0 :!label _label)
      (Variables|Default|SetDamage 1.5e+02))
    (:1
      (Variables|Default|SetBurnDuration 3.0)
      (Variables|Default|SetDamage 6e+01))
    (:2
      (Variables|Default|SetBurnDuration 4.0)
      (Variables|Default|SetDamage 9e+01))
    (:3
      (goto _label)))
  (bind _outhits (Class|KismetSystemLibrary|LineTraceMultiforObjects (Transformation|GetActorLocation) (Transformation|GetActorLocation TargetingUnit) (Utilities|Array|MakeArray "ObjectTypeQuery1" "ObjectTypeQuery2" "ObjectTypeQuery3") false 0 "ForDuration" true))
  (for _array_element _outhits
    (bind _asbp_combat_unit_base (Utilities|Casting|CastToBP_CombatUnitBase (.HitActor (Collision|BreakHitResult _array_element))))
    (Utilities|IsValid _asbp_combat_unit_base
      (:Is%20Valid
        (Default|AlterHP _asbp_combat_unit_base (Variables|Default|GetDamage))
        (Variables|/Game/Blueprints/Gameplay/Units/BP_CombatUnitBase.BP_CombatUnitBase_C|SetBurningTimer _asbp_combat_unit_base (Variables|Default|GetBurnDuration))))))

(fn ConstructionScript
  (|CallParentFunction))