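; BP_TestUnit4 is a test unit variant whose ability is a timed health regeneration on itself.
; CastAbility sets the regen duration and rate by Tier, with stronger values at higher tiers and any unlisted tier sharing the tier 3 values.
; While time remains, Tick applies the rate through AlterHP scaled by frame time, counts the timer down, then calls the parent Tick.
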(event EventBeginPlay
  (|CallParentFunction) ; This node is disabled and will not be called.\nDrag off pins to build functionality.
)

(event Collision|EventActorBeginOverlap
  (params (OtherActor :type Actor%20Object%20Reference)))

(event EventTick
  (params (DeltaSeconds :type Float%20%28single-precision%29))
  (if (> (Variables|Default|GetRegenFor) 0.0)
    (CallFunction|AlterHP (* (Variables|Default|GetRegenRate) DeltaSeconds))
    (Variables|Default|SetRegenFor (- (Variables|Default|GetRegenFor) (Utilities|Time|GetWorldDeltaSeconds))))
  (|CallParentFunction DeltaSeconds))

(event EventCastAbility
  (params (TargetingUnit :type BP%20Combat%20Unit%20Base%20Object%20Reference))
  (switch int (Variables|Default|GetTier)
    (:Default
      (Variables|Default|SetRegenFor 7.0 :!label _label)
      (Variables|Default|SetRegenRate 3e+01))
    (:1
      (Variables|Default|SetRegenFor 5.0)
      (Variables|Default|SetRegenRate 1e+01))
    (:2
      (Variables|Default|SetRegenFor 6.0)
      (Variables|Default|SetRegenRate 2e+01))
    (:3
      (goto _label))))

(fn ConstructionScript
  (|CallParentFunction))