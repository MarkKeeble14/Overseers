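; BP_TestUnit5 is a unit variant whose cast ability emits a radial pulse around itself.
; CastAbility sets pulse damage and radius by Tier, with tier 3 and any unlisted tier sharing the strongest values.
; A sphere overlap then passes the damage to AlterHP on every other BP_CombatUnitBase in range, with no team check.
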(event EventBeginPlay
  (|CallParentFunction) ; This node is disabled and will not be called.\nDrag off pins to build functionality.
)

(event Collision|EventActorBeginOverlap
  (params (OtherActor :type Actor%20Object%20Reference)))

(event EventTick
  (params (DeltaSeconds :type Float%20%28single-precision%29))
  (|CallParentFunction DeltaSeconds) ; This node is disabled and will not be called.\nDrag off pins to build functionality.
)

(event EventCastAbility
  (params (TargetingUnit :type BP%20Combat%20Unit%20Base%20Object%20Reference))
  (switch int (Variables|Default|GetTier)
    (:Default
      (Variables|Default|SetPulseDamage 1e+02 :!label _label)
      (Variables|Default|SetPulseRange 7.5e+02))
    (:1
      (Variables|Default|SetPulseDamage 5e+01)
      (Variables|Default|SetPulseRange 5e+02))
    (:2
      (Variables|Default|SetPulseDamage 75.0)
      (Variables|Default|SetPulseRange 6e+02))
    (:3
      (goto _label)))
  (bind _outactors (Collision|SphereOverlapActors (Transformation|GetActorLocation) (Variables|Default|GetPulseRange) (Utilities|Array|MakeArray "ObjectTypeQuery1" "ObjectTypeQuery2" "ObjectTypeQuery3") "/Game/Blueprints/Gameplay/Units/BP_CombatUnitBase.BP_CombatUnitBase_C" (Utilities|Array|MakeArray self)))
  (for _array_element _outactors
    (bind _asbp_combat_unit_base (Utilities|Casting|CastToBP_CombatUnitBase _array_element))
    (Utilities|IsValid _asbp_combat_unit_base
      (:Is%20Valid
        (Default|AlterHP _asbp_combat_unit_base (Variables|Default|GetPulseDamage))))))

(fn ConstructionScript
  (|CallParentFunction))