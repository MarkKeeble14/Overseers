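; BP_TestUnit1 is a test unit variant whose cast ability grants a shield that scales with the unit's Tier.
; CastAbility switches on Tier to choose the AddShield amount, with unmatched tiers getting the same amount as the third tier.
; Every branch then calls MC_StartCastMontage, an event named as a multicast, which plays the unit's cast montage on its Mesh.
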(event Custom|MC_StartCastMontage
  (Animation|Montage|PlayMontage (Variables|Character|GetMesh) "/Game/Characters/Units/TestUnit1/Animations/Montage_TestUnit1Cast.Montage_TestUnit1Cast"))

(event EventBeginPlay
  (|CallParentFunction) ; This node is disabled and will not be called.\nDrag off pins to build functionality.
)

(event Collision|EventActorBeginOverlap
  (params (OtherActor :type Actor%20Object%20Reference)))

(event EventTick
  (params (DeltaSeconds :type Float%20%28single-precision%29))
  (|CallParentFunction DeltaSeconds) ; This node is disabled and will not be called.\nDrag off pins to build functionality.
)

(event EventCastAbility
  (params (TargetingUnit :type BP%20Combat%20Unit%20Base%20Object%20Reference))
  (switch int (Variables|Default|GetTier)
    (:Default
      (CallFunction|AddShield 1e+02 :!label _label))
    (:1
      (CallFunction|AddShield 25.0))
    (:2
      (CallFunction|AddShield 5e+01))
    (:3
      (goto _label)))
  (CallFunction|MCStartCastMontage))

(fn ConstructionScript
  (|CallParentFunction))