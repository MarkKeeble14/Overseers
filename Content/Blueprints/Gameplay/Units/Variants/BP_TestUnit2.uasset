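; BP_TestUnit2 is a test unit variant whose cast ability raises its own HP by an amount set by its Tier.
; CastAbility switches on Tier and calls AlterHP, with tier 3 and any unlisted tier sharing the largest amount.
; Every branch then calls MC_StartCastMontage, which plays the unit's cast montage on its mesh.
; BeginPlay is disabled, while Tick and the construction script only call the parent.
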(event Custom|MC_StartCastMontage
  (Animation|Montage|PlayMontage (Variables|Character|GetMesh) "/Game/Characters/Units/TestUnit2/Animations/Montage_TestUnit2Cast.Montage_TestUnit2Cast"))

(event EventBeginPlay
  (|CallParentFunction) ; This node is disabled and will not be called.\nDrag off pins to build functionality.
)

(event Collision|EventActorBeginOverlap
  (params (OtherActor :type Actor%20Object%20Reference)))

(event EventTick
  (params (DeltaSeconds :type Float%20%28single-precision%29))
  (|CallParentFunction DeltaSeconds))

(event EventCastAbility
  (params (TargetingUnit :type BP%20Combat%20Unit%20Base%20Object%20Reference))
  (switch int (Variables|Default|GetTier)
    (:Default
      (CallFunction|AlterHP 5e+01 :!label _label))
    (:1
      (CallFunction|AlterHP 15.0))
    (:2
      (CallFunction|AlterHP 3e+01))
    (:3
      (goto _label)))
  (CallFunction|MCStartCastMontage))

(fn ConstructionScript
  (|CallParentFunction))