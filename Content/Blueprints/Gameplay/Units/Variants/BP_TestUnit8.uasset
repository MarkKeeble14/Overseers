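; Test combat unit variant whose ability sends a chaining radial pulse out from the targeted unit.
; CastAbility sets chain count and pulse damage by Tier, then starts PulseAroundUnit with itself excluded.
; Each pulse sphere-overlaps nearby combat units, calls AlterHP and recurses from each while chains remain.
; As wired, AlterHP receives zero instead of PulseDamage and recursion passes zero chains, limiting it to one hop.
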(event Custom|PulseAroundUnit
  (params (TargetingUnit :type BP%20Combat%20Unit%20Base%20Object%20Reference) (HitActors :type Array%20of%20Actor%20Object%20References) (ChainsRemaining :type Integer))
  (Utilities|IsValid TargetingUnit
    (:Is%20Valid
      (bind _outactors (Collision|SphereOverlapActors (Transformation|GetActorLocation TargetingUnit) 5e+02 (Utilities|Array|MakeArray "ObjectTypeQuery1" "ObjectTypeQuery2" "ObjectTypeQuery3") "/Game/Blueprints/Gameplay/Units/BP_CombatUnitBase.BP_CombatUnitBase_C" HitActors))
      (for _array_element _outactors
        (bind _asbp_combat_unit_base (Utilities|Casting|CastToBP_CombatUnitBase _array_element))
        (Utilities|IsValid _asbp_combat_unit_base
          (:Is%20Valid
            (Default|AlterHP _asbp_combat_unit_base 0.0)
            (if (> ChainsRemaining 0)
              (Utilities|Array|Add HitActors _asbp_combat_unit_base)
              (CallFunction|PulseAroundUnit _asbp_combat_unit_base HitActors))))))))

(event EventBeginPlay
  (|CallParentFunction) ; This node is disabled and will not be called.\nDrag off pins to build functionality.
)

(event Collision|EventActorBeginOverlap
  (params (OtherActor :type Actor%20Object%20Reference)))

(event EventTick
  (params (DeltaSeconds :type Float%20%28single-precision%29))
  (|CallParentFunction DeltaSeconds))

(event EventCastAbility
  (params (TargetingUnit :type BP%20Combat%20Unit%20Base%20Object%20Reference))
  (switch int (Variables|Default|GetTier)
    (:Default
      (Variables|Default|SetTimesCanChain 5 :!label _label)
      (Variables|Default|SetPulseDamage 6e+01))
    (:1
      (Variables|Default|SetTimesCanChain 2)
      (Variables|Default|SetPulseDamage 2e+01))
    (:2
      (Variables|Default|SetTimesCanChain 3)
      (Variables|Default|SetPulseDamage 4e+01))
    (:3
      (goto _label)))
  (CallFunction|PulseAroundUnit TargetingUnit (Utilities|Array|MakeArray self) (Variables|Default|GetTimesCanChain)))

(fn ConstructionScript
  (|CallParentFunction))