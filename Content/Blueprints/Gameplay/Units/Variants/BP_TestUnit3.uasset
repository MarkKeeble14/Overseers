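; Test unit variant, by its name, whose CastAbility applies a tier-scaled HP change and plays a cast montage.
; After a short delay, it calls AlterHP with a negative AttackDamage multiple that grows with Tier.
; Only tier 1 calls it on TargetingUnit; other tiers call it on the unit itself.
; All branches then trigger the montage through MC_StartMontage, named as a multicast.
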(event Custom|MC_StartMontage
  (Animation|Montage|PlayMontage (Variables|Character|GetMesh) "/Game/Characters/Units/TestUnit3/Animations/Montage_TestUnit3Cast.Montage_TestUnit3Cast"))

(event EventBeginPlay
  (|CallParentFunction) ; This node is disabled and will not be called.\nDrag off pins to build functionality.
)

(event Collision|EventActorBeginOverlap
  (params (OtherActor :type Actor%20Object%20Reference)))

(event EventTick
  (params (DeltaSeconds :type Float%20%28single-precision%29))
  (|CallParentFunction DeltaSeconds))

(event EventCastAbility
  (params (TargetingUnit :type BP%20Combat%20Unit%20Base%20Object%20Reference))
  (Utilities|FlowControl|Delay 0.75)
  (switch int (Variables|Default|GetTier)
    (:Default
      (CallFunction|AlterHP (* (Variables|Default|GetAttackDamage) -6.0) :!label _label))
    (:1
      (Default|AlterHP TargetingUnit (* (Variables|Default|GetAttackDamage) -3.0)))
    (:2
      (CallFunction|AlterHP (* (Variables|Default|GetAttackDamage) -4.0)))
    (:3
      (goto _label)))
  (CallFunction|MCStartMontage))

(fn ConstructionScript
  (|CallParentFunction))