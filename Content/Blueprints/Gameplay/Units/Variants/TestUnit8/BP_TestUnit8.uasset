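; BP_TestUnit8 is a unit variant whose cast ability releases a damaging, chain-capable pulse centered on the targeted unit.
; CastAbility scales chain count, damage and radius by Tier, with tier 3 sharing the default values.
; An S_ event spawns a tiny BP_PulseBall carrying those values and owner ID, ignoring target and caster.
; An MC_ event plays the cast montage and re-enables attacking on completion.
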(event Custom|S_SpawnSphereAroundUnit
  (params (CanChain :type Integer) (Damage :type Float%20%28double-precision%29) (Range :type Float%20%28double-precision%29) (HittingUnit :type BP%20Combat%20Unit%20Base%20Object%20Reference))
  (bind _returnvalue (Game|SpawnActorfromClass "/Game/Blueprints/Gameplay/Units/Variants/TestUnit8/BP_PulseBall.BP_PulseBall_C" (Math|Transform|MakeTransform (Transformation|GetActorLocation HittingUnit) "0, 0, 0" "0.010000,0.010000,0.010000") "Undefined" "MultiplyWithRoot" 0 0))
  (Variables|/Game/Blueprints/Gameplay/Units/Variants/TestUnit8/BP_PulseBall.BP_PulseBall_C|SetMaxScale _returnvalue Range)
  (Variables|/Game/Blueprints/Gameplay/Units/Variants/TestUnit8/BP_PulseBall.BP_PulseBall_C|SetDamage _returnvalue Damage)
  (Variables|/Game/Blueprints/Gameplay/Units/Variants/TestUnit8/BP_PulseBall.BP_PulseBall_C|SetCanChain _returnvalue CanChain)
  (Variables|/Game/Blueprints/Gameplay/Units/Variants/TestUnit8/BP_PulseBall.BP_PulseBall_C|SetIgnoreActors _returnvalue (Utilities|Array|MakeArray HittingUnit self))
  (Variables|/Game/Blueprints/Gameplay/Units/Variants/TestUnit8/BP_PulseBall.BP_PulseBall_C|SetSpawnedByPlayerId _returnvalue (Variables|Default|GetOwnedByPlayerID)))

(event Custom|MC_StartCastMontage
  (Animation|Montage|PlayMontage (Variables|Character|GetMesh) "/Game/Characters/Units/TestUnit8/Animations/Montage_TestUnit8Cast.Montage_TestUnit8Cast"
    (:OnCompleted
      (Variables|Default|SetCanAttack true))))

(event EventBeginPlay
  (|CallParentFunction) ; This node is disabled and will not be called.\nDrag off pins to build functionality.
)

(event Collision|EventActorBeginOverlap
  (params (OtherActor :type Actor%20Object%20Reference)))

(event EventTick
  (params (DeltaSeconds :type Float%20%28single-precision%29))
  (|CallParentFunction DeltaSeconds))

(event EventCastAbility
  (params (TargetingUnit :type BP%20Combat%20Unit%20Base%20Object%20Reference))
  (switch int (Variables|Default|GetTier)
    (:Default
      (Variables|Default|SetTimesCanChain 5 :!label _label)
      (Variables|Default|SetPulseDamage 1e+02)
      (Variables|Default|SetPulseRadius 5e+01))
    (:1
      (Variables|Default|SetTimesCanChain 2)
      (Variables|Default|SetPulseDamage 4e+01)
      (Variables|Default|SetPulseRadius 15.0))
    (:2
      (Variables|Default|SetTimesCanChain 3)
      (Variables|Default|SetPulseDamage 6e+01)
      (Variables|Default|SetPulseRadius 25.0))
    (:3
      (goto _label)))
  (CallFunction|SSpawnSphereAroundUnit (Variables|Default|GetTimesCanChain) (Variables|Default|GetPulseDamage) (Variables|Default|GetPulseRadius) TargetingUnit)
  (CallFunction|MCStartCastMontage))

(fn ConstructionScript
  (|CallParentFunction))