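; BP_PulseBall is an expanding pulse from a unit variant that damages overlapping enemy combat units and chains outward from them.
; Tick grows the actor's scale, and the server destroys it once it reaches MaxScale.
; On server overlap it applies damage and, while CanChain remains, spawns a copy at the victim with one fewer chain.
; An inherited IgnoreActors list gates further spawns, though not the damage itself.
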(event EventBeginPlay)

(event Collision|EventActorBeginOverlap
  (params (OtherActor :type Actor%20Object%20Reference))
  (Networking|SwitchHasAuthority
    (:Authority
      (if (> (Variables|Default|GetCanChain) 0)
        (bind _asbp_combat_unit_base (Utilities|Casting|CastToBP_CombatUnitBase OtherActor))
        (Utilities|IsValid _asbp_combat_unit_base
          (:Is%20Valid
            (if (!= (Variables|/Game/Blueprints/Gameplay/Units/BP_BaseUnit.BP_BaseUnit_C|GetOwnedByPlayerID _asbp_combat_unit_base) (Variables|Default|GetSpawnedByPlayerId))
              (Default|AlterHP _asbp_combat_unit_base (* (Variables|Default|GetDamage) -1.0))
              (if (not (Utilities|Array|ContainsItem (Variables|Default|GetIgnoreActors) 0))
                (bind _returnvalue (Game|SpawnActorfromClass "BP_PulseBall_C" (Math|Transform|MakeTransform (Transformation|GetActorLocation _asbp_combat_unit_base) "0, 0, 0" "1.000000,1.000000,1.000000") "Undefined" "MultiplyWithRoot" 0 0))
                (Variables|BP_PulseBall_C|SetDamage _returnvalue (Variables|Default|GetDamage))
                (Variables|BP_PulseBall_C|SetMaxScale _returnvalue (Variables|Default|GetMaxScale))
                (Utilities|Array|Add (Variables|Default|GetIgnoreActors) _asbp_combat_unit_base)
                (Variables|BP_PulseBall_C|SetIgnoreActors _returnvalue (Variables|Default|GetIgnoreActors))
                (bind _output_get (Variables|BP_PulseBall_C|SetCanChain _returnvalue (- (Variables|Default|GetCanChain) 1)))
                (Variables|BP_PulseBall_C|SetSpawnedByPlayerId _returnvalue (Variables|Default|GetSpawnedByPlayerId))
                (Development|PrintString (Utilities|String|ToString(Integer) _output_get))))))))))

(event EventTick
  (params (DeltaSeconds :type Float%20%28single-precision%29))
  (bind _returnvalue (Transformation|GetActorScale3D))
  (bind _pulsespeed (Variables|Default|GetPulseSpeed))
  (bind _returnvalue_2 (* DeltaSeconds _pulsespeed))
  (bind _returnvalue_3 (+ _returnvalue _returnvalue_2))
  (Transformation|SetActorScale3D _returnvalue_3)
  (Networking|SwitchHasAuthority
    (:Authority
      (if (>= (.X (Math|Vector|BreakVector _returnvalue_3)) (Variables|Default|GetMaxScale))
        (Actor|DestroyActor)))))

(fn ConstructionScript)