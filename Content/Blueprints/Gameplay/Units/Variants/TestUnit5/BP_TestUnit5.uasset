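; TestUnit5 is a unit variant whose cast ability is a ground-pound pulse with damage and range set by its Tier.
; CastAbility picks those values, with unmatched tiers sharing the top-tier numbers, then calls the MC_ effect and S_ spawn events.
; The effect event plays Niagara and a cast montage, restoring CanAttack on completion.
; The spawn event creates a tiny BP_PoundCylinder, passing it the owning player, damage and maximum scale.
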(event Custom|MC_SpawnSystem
  (Niagara|SpawnSystematLocation "/Game/Blueprints/Gameplay/Units/Variants/TestUnit5/Niagra_Pound.Niagra_Pound" (Transformation|GetActorLocation))
  (Animation|Montage|PlayMontage (Variables|Character|GetMesh) "/Game/Characters/Units/TestUnit5/Animations/Montage_TestUnit5Cast.Montage_TestUnit5Cast"
    (:OnCompleted
      (Variables|Default|SetCanAttack true))))

(event Custom|S_SpawnPound
  (bind _returnvalue (Game|SpawnActorfromClass "/Game/Blueprints/Gameplay/Units/Variants/TestUnit5/BP_PoundCylinder.BP_PoundCylinder_C" (Math|Transform|MakeTransform (Transformation|GetActorLocation) "0, 0, 0" "0.010000,0.010000,0.010000") "Undefined" "MultiplyWithRoot" 0 0))
  (Variables|/Game/Blueprints/Gameplay/Units/Variants/TestUnit5/BP_PoundCylinder.BP_PoundCylinder_C|SetSpawnedByPlayerID _returnvalue (Variables|Default|GetOwnedByPlayerID))
  (Variables|/Game/Blueprints/Gameplay/Units/Variants/TestUnit5/BP_PoundCylinder.BP_PoundCylinder_C|SetDamage _returnvalue (Variables|Default|GetPulseDamage))
  (Variables|/Game/Blueprints/Gameplay/Units/Variants/TestUnit5/BP_PoundCylinder.BP_PoundCylinder_C|SetMaxScale _returnvalue (Variables|Default|GetPulseRange)))

(event EventBeginPlay
  (|CallParentFunction) ; This node is disabled and will not be called.\nDrag off pins to build functionality.
)

(event Collision|EventActorBeginOverlap
  (params (OtherActor :type Actor%20Object%20Reference)))

(event EventTick
  (params (DeltaSeconds :type Float%20%28single-precision%29))
  (|CallParentFunction DeltaSeconds) ; This node is disabled and will not be called.\nDrag off pins to build functionality.
)

(event EventCastAbility
  (params (TargetingUnit :type BP%20Combat%20Unit%20Base%20Object%20Reference))
  (switch int (Variables|Default|GetTier)
    (:Default
      (Variables|Default|SetPulseDamage 1.5e+02 :!label _label)
      (Variables|Default|SetPulseRange 5e+01))
    (:1
      (Variables|Default|SetPulseDamage 75.0)
      (Variables|Default|SetPulseRange 25.0))
    (:2
      (Variables|Default|SetPulseDamage 1e+02)
      (Variables|Default|SetPulseRange 35.0))
    (:3
      (goto _label)))
  (CallFunction|MCSpawnSystem)
  (CallFunction|SSpawnPound))

(fn ConstructionScript
  (|CallParentFunction))