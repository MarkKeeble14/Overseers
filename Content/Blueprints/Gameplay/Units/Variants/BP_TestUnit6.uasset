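; Test unit variant whose CastAbility deals a timed three-hit combo to a targeted unit.
; The unit's Tier selects a bonus added to AttackDamage, then MC_StartMontage plays the cast animation on its mesh.
; Chained delays time the hits at one, two and three times the boosted damage through AlterHP, continuing only while the target is alive.
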(event Custom|MC_StartMontage
  (Animation|Montage|PlayMontage (Variables|Character|GetMesh) "/Game/Characters/Units/TestUnit6/Animations/Montage_TestUnit6Cast.Montage_TestUnit6Cast"))

(event EventBeginPlay
  (|CallParentFunction) ; This node is disabled and will not be called.\nDrag off pins to build functionality.
)

(event Collision|EventActorBeginOverlap
  (params (OtherActor :type Actor%20Object%20Reference)))

(event EventTick
  (params (DeltaSeconds :type Float%20%28single-precision%29))
  (|CallParentFunction DeltaSeconds) ; This node is disabled and will not be called.\nDrag off pins to build functionality.
)

(event EventCastAbility
  (params (TargetingUnit :type BP%20Combat%20Unit%20Base%20Object%20Reference))
  (switch int (Variables|Default|GetTier)
    (:1
      (Variables|Default|SetDamageIncrease 5.0))
    (:2
      (Variables|Default|SetDamageIncrease 15.0))
    (:3
      (Variables|Default|SetDamageIncrease 45.0)))
  (CallFunction|MCStartMontage)
  (Utilities|FlowControl|Delay 0.75)
  (Default|AlterHP TargetingUnit (* (+ (Variables|Default|GetAttackDamage) (Variables|Default|GetDamageIncrease)) -1.0))
  (if (Variables|/Game/Blueprints/Gameplay/Units/BP_CombatUnitBase.BP_CombatUnitBase_C|GetAlive TargetingUnit)
    (Utilities|FlowControl|Delay 0.4)
    (Default|AlterHP TargetingUnit (* (+ (Variables|Default|GetAttackDamage) (Variables|Default|GetDamageIncrease)) -2.0))
    (if (Variables|/Game/Blueprints/Gameplay/Units/BP_CombatUnitBase.BP_CombatUnitBase_C|GetAlive TargetingUnit)
      (Utilities|FlowControl|Delay 0.8)
      (Default|AlterHP TargetingUnit (* (+ (Variables|Default|GetAttackDamage) (Variables|Default|GetDamageIncrease)) -3.0))
      (if (Variables|/Game/Blueprints/Gameplay/Units/BP_CombatUnitBase.BP_CombatUnitBase_C|GetAlive TargetingUnit)
        _))))

(fn ConstructionScript
  (|CallParentFunction))