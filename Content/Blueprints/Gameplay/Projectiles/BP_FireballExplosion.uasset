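; BP_FireballExplosion is an expanding explosion actor for fireball projectiles, with no damage or collision logic in its graphs.
; Every Tick adds PulseSpeed scaled by delta time to the actor's scale on each machine running it.
; Only the authority destroys it, once X scale reaches MaxScale.
; That check re-evaluates the sum after scaling, so it tests one step ahead of the applied scale.
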(event EventTick
  (params (DeltaSeconds :type Float%20%28single-precision%29))
  (bind _returnvalue (Transformation|GetActorScale3D))
  (bind _pulsespeed (Variables|Default|GetPulseSpeed))
  (bind _returnvalue_2 (* DeltaSeconds _pulsespeed))
  (bind _returnvalue_3 (+ _returnvalue _returnvalue_2))
  (Transformation|SetActorScale3D _returnvalue_3)
  (Networking|SwitchHasAuthority
    (:Authority
      (if (>= (.X (Math|Vector|BreakVector _returnvalue_3)) (Variables|Default|GetMaxScale))
        (Actor|DestroyActor)))))

(fn ConstructionScript)