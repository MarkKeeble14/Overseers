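; Projectile actor that sets a uniform scale on itself and destroys itself after a fixed lifetime.
; BeginPlay applies StartScale, then waits on a Delay before calling DestroyActor.
; Tick sets scale to a lerp from StartScale to MaxScale using LerpSpeed directly as alpha, so the result does not accumulate over time.
; The graphs contain no movement or hit logic.
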(event EventBeginPlay
  (bind _startscale (Variables|Default|GetStartScale))
  (Transformation|SetActorScale3D (Math|Vector|MakeVector _startscale _startscale _startscale))
  (Utilities|FlowControl|Delay 15.0)
  (Actor|DestroyActor))

(event Collision|EventActorBeginOverlap
  (params (OtherActor :type Actor%20Object%20Reference)))

(event EventTick
  (params (DeltaSeconds :type Float%20%28single-precision%29))
  (bind _maxscale (Variables|Default|GetMaxScale))
  (bind _startscale (Variables|Default|GetStartScale))
  (Transformation|SetActorScale3D (Math|Vector|Lerp(Vector) (Math|Vector|MakeVector _startscale _startscale _startscale) (Math|Vector|MakeVector _maxscale _maxscale _maxscale) (Variables|Default|GetLerpSpeed))))

(fn ConstructionScript)